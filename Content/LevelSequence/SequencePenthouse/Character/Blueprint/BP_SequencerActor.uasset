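; Sequencer character actor whose skeletal mesh, audio and decal respond to the camera's active filter.
; Gets its managers through the SceneManager singleton, then polls CameraManager's filter on Tick: audio is audible only in AUDIO, custom depth renders only in THERMAL.
; PlayAudio shows the decal; non-audio filters hide it.
; The filter-change handler is empty, and the sequence play/pause binding never runs.
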(event Custom|BindChangeFilter
  (EventDispatchers|BindEventtoOnChangeFilter (Variables|/Game/Blueprint/Global/Manager/BP_SceneManager.BP_SceneManager_C|GetCameraManager (Variables|Default|GetScene%20Manager)) (delegate Custom|OnChangeFilter)))

(event Custom|OnChangeFilter
  (params (SelectedFilter :type EFilterType%20Enum :default "NewEnumerator0") (PostProcessIndex :type Integer)))

(event Custom|ThermalRender
  (params (bValue :type Boolean))
  (Rendering|SetRenderCustomDepth (Variables|Default|GetSkeletalMesh) bValue))

(event Custom|OnPlaySequence_Event
  (params (Play/Pause :type EPlaySequence%20Enum :default "NewEnumerator0"))
  (switch Utilities|FlowControl|Switch|SwitchonEPlaySequence Play/Pause
    (:NewEnumerator1
      (CallFunction|UnpauseAudio))
    (:NewEnumerator2
      (CallFunction|PauseAudio))))

(event Custom|BindSequenceControl)

(event Custom|PauseAudio
  (Class|AudioComponent|SetPaused (Variables|Default|GetAudio) true))

(event Custom|UnpauseAudio
  (Class|AudioComponent|SetPaused (Variables|Default|GetAudio) false))

(event Custom|BindInit
  ;[1 1 1] Initialization Binding Event
  (bind _output_get (Variables|Default|SetScene%20Manager (.AsBP%20Scene%20Manager (Utilities|Casting|CastToBP_SceneManager (CallFunction|GetSingletonInstance "/Game/Blueprint/Global/Manager/BP_SceneManager.BP_SceneManager_C")))))
  (EventDispatchers|BindEventtoOnInitializationBind _output_get (delegate Custom|BindInitEvent)))

(event Custom|BindInitEvent
  ;[1 1 1] Initialization Binding Event
  (Utilities|FlowControl|Sequence
    (:then_0
      (CallFunction|SetManagerVariable))
    (:then_1
      (CallFunction|BindAllEvent))))

(event Custom|PlayAudio
  (params (NewSound :type Sound%20Base%20Object%20Reference))
  (bind _audio (Variables|Default|GetAudio))
  ;[1 1 1] Set Audio Play and Volume
  (Audio|Components|Audio|SetSound _audio NewSound)
  (Audio|Components|Audio|Play _audio 0.0)
  (CallFunction|VisibleDecal))

(event Custom|StopAudio
  ;[1 1 1] Set Audio Play and Volume
  (Audio|Components|Audio|Stop (Variables|Default|GetAudio))
  (CallFunction|MuteAudio)
  (CallFunction|HiddeDecal))

(event Custom|MuteAudio
  (Audio|Components|Audio|SetVolumeMultiplier (Variables|Default|GetAudio) 0.0 :!class /Script/Engine.AudioComponent))

(event Custom|UnmuteAudio
  (Audio|Components|Audio|SetVolumeMultiplier (Variables|Default|GetAudio) 1.0 :!class /Script/Engine.AudioComponent))

(event Custom|HiddeDecal
  ;[1 1 1] Set Visibility Decal Filter
  (Rendering|SetVisibility (Variables|Default|GetDecal) false false))

(event Custom|VisibleDecal
  ;[1 1 1] Set Visibility Decal Filter
  (Rendering|SetVisibility (Variables|Default|GetDecal) true false))

(event EventBeginPlay
  ;[1 1 1] Initialization Binding Event
  (CallFunction|BindInit))

(event EventTick
  (params (DeltaSeconds :type Float%20%28single-precision%29))
  (bind _camera_manager (Variables|Default|GetCamera%20Manager))
  (Utilities|IsValid _camera_manager
    (:Is%20Valid
      (switch Utilities|FlowControl|Switch|SwitchonEFilterType (Variables|/Game/Blueprint/Global/Manager/BP_CameraManager.BP_CameraManager_C|GetCurrentFilter _camera_manager)
        (:NewEnumerator0
          (CallFunction|MuteAudio :!label _label)
          (CallFunction|HiddeDecal)
          (CallFunction|ThermalRender false :!label _label_2))
        (:NewEnumerator1
          (CallFunction|UnmuteAudio)
          (Development|PrintString (Utilities|String|EnumtoString (Audio|Components|Audio|GetPlayState (Variables|Default|GetAudio))) true true "(R=0.000000,G=0.660000,B=1.000000,A=1.000000)" 2.0 "f")
          (goto _label_2))
        (:NewEnumerator2
          (CallFunction|ThermalRender true)
          (CallFunction|MuteAudio)
          (CallFunction|HiddeDecal))
        (:NewEnumerator3
          (goto _label))))))

(fn ConstructionScript)

(fn BindAllEvent
  (CallFunction|BindChangeFilter))

(fn SetManagerVariable
  (bind _scene_manager (Variables|Default|GetScene%20Manager))
  (Utilities|FlowControl|Sequence
    (:then_0
      (Variables|Default|SetSequencer%20Manager (Variables|/Game/Blueprint/Global/Manager/BP_SceneManager.BP_SceneManager_C|GetSequencerManager _scene_manager))
      (Variables|Default|SetCamera%20Manager (Variables|/Game/Blueprint/Global/Manager/BP_SceneManager.BP_SceneManager_C|GetCameraManager _scene_manager)))))