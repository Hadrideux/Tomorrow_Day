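; Player controller that switches between the player character and a photo mode, and manages the photo gallery.
; The photo input spawns a BP_PhotoController at the camera and possesses it, or destroys it, repossesses the character and re-adds the action mapping context.
; Taken photos feed an array passed to the W_Bracelet widget, which opens only during photo mode.
; Bracelet movement and Add/Subtract keys forward to a unique BP_PlayerCharacterController instance.
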(event Custom|InputPlayer
  (bind _asplayer_controller (Utilities|Casting|CastToPlayerController (Pawn|GetController (Variables|Default|GetPlayerCharacter))))
  (Utilities|IsValid (PlayerController|LocalPlayerSubsystems|GetEnhancedInputLocalPlayerSubsystem _asplayer_controller)
    (:Is%20Valid
      (Input|AddMappingContext (PlayerController|LocalPlayerSubsystems|GetEnhancedInputLocalPlayerSubsystem _asplayer_controller) "/Game/Blueprint/Character/InputAction/IMC_PlayerAction.IMC_PlayerAction" 0 "(bIgnoreAllPressedKeysUntilRelease=True,bForceImmediately=False)"))))

(event Custom|AddToGallery
  (params (Photo :type Texture%20Render%20Target%202D%20Object%20Reference))
  (Utilities|Array|Add (Variables|Default|GetPhotoGallery) Photo))

(event Input|EnhancedActionEvents|EnhancedInputActionIA_PlayerPhoto
  (params (ActionValue :type Boolean) (ElapsedSeconds :type Float%20%28double-precision%29) (TriggeredSeconds :type Float%20%28double-precision%29) (InputAction :type Input%20Action%20Object%20Reference :default "/Game/Blueprint/Character/InputAction/PlayerAction/IA_PlayerPhoto.IA_PlayerPhoto"))
  (:Started
    (Variables|Default|GetModePhoto
      (:then
        (Pawn|UnPossess)
        (Pawn|Possess (Variables|Default|GetPlayerCharacter))
        (Actor|DestroyActor (Variables|Default|GetModePhoto))
        (CallFunction|InputPlayer))
      (:else
        (bind _returnvalue (Game|SpawnActorfromClass "/Game/Blueprint/PhotoMode/BP_PhotoController.BP_PhotoController_C" (Transformation|GetActorTransform (Game|GetPlayerCameraManager 0)) "Undefined" 0 0))
        (bind _output_get (Variables|Default|SetModePhoto _returnvalue))
        (Pawn|UnPossess)
        (Pawn|Possess _output_get)
        (EventDispatchers|BindEventtoTakenPhoto _output_get (delegate Custom|AddToGallery))))))

(event Input|EnhancedActionEvents|EnhancedInputActionIA_PlayerBracelet
  (params (ActionValue :type Boolean) (ElapsedSeconds :type Float%20%28double-precision%29) (TriggeredSeconds :type Float%20%28double-precision%29) (InputAction :type Input%20Action%20Object%20Reference :default "/Game/Blueprint/Character/InputAction/PlayerAction/IA_PlayerBracelet.IA_PlayerBracelet"))
  (:Started
    (Default|MoveBracelet (Variables|Default|GetCharacterController))
    (bind _gallery (Variables|Default|GetGallery)
      (:then
        (Widget|RemovefromParent _gallery)
        (Variables|Default|SetGallery 0))
      (:else
        (Variables|Default|GetModePhoto
          (:then
            (bind _returnvalue (UserInterface|CreateWidget "/Game/Blueprint/UI_Blueprint/InGame/W_Bracelet.W_Bracelet_C" 0 (Variables|Default|GetPhotoGallery)))
            (bind _output_get (Variables|Default|SetGallery _returnvalue))
            (UserInterface|Viewport|AddtoViewport _output_get 0))
          (:else))))))

(event EventBeginPlay
  (Variables|Default|SetPlayerCharacter (Game|GetPlayerCharacter 0))
  (bind _asbp_player_character_controller (Utilities|Casting|CastToBP_PlayerCharacterController (CallFunction|GetUniqueInstance "/Game/Blueprint/Character/BP_PlayerCharacterController.BP_PlayerCharacterController_C")))
  (Variables|Default|SetCharacterController _asbp_player_character_controller))

(event Input|KeyboardEvents|Add
  (params (Key :type Key%20Structure :default "None"))
  (:Pressed
    (Default|Add (Variables|Default|GetCharacterController))))

(event Input|KeyboardEvents|Subtract
  (params (Key :type Key%20Structure :default "None"))
  (:Pressed
    (Default|Remove (Variables|Default|GetCharacterController))))

(fn ConstructionScript)