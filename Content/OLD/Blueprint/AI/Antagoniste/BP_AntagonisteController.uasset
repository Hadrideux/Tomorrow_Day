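; BP_AntagonisteController is an AI antagonist that chases the player and triggers game over on reaching them.
; On BeginPlay it caches the BP_UIManager unique instance, then starts the chase after a short delay.
; AI MoveTo runs on itself toward the player character, calling SetGameOver on the UI manager on success and retrying on failure.
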(event Custom|MoveTo
  ;[1 1 1] IA Set Destination Move To
  (AI|AIMoveTo self "0, 0, 0" (Game|GetPlayerCharacter 0) 5.0 false
    (:OnSuccess
      (Default|SetGameOver (Variables|Default|GetUIManager)))
    (:OnFail
      (CallFunction|Moveto))))

(event EventBeginPlay
  (Utilities|FlowControl|Sequence
    (:then_0
      (bind _asbp_uimanager (Utilities|Casting|CastToBP_UIManager (CallFunction|GetUniqueInstance "/Game/Blueprint/UI_Blueprint/BP_UIManager.BP_UIManager_C")))
      (Variables|Default|SetUIManager _asbp_uimanager))
    (:then_1
      (Utilities|FlowControl|Delay 0.2)
      (CallFunction|Moveto))))

(fn ConstructionScript)