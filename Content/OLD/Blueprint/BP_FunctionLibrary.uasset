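; BP_FunctionLibrary is a set of shared helper functions, mainly for looking up single-instance actors by class.
; GetUniqueInstance checks the ObjectClass map, fills a missing entry through GetActorOfClass, then returns the mapped actor.
; CreateWidget has an empty body, with unconnected nodes left over for creating menu, game over, pause and map description widgets.
; TimeLineLerped is an empty stub.
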(fn GetUniqueInstance
  (params (ObjectActor :type Actor%20Class%20Reference))
  (bind _object_class (LocalVariables|GetObject%20Class))
  (bind (_value _returnvalue) (Utilities|Map|Find _object_class ObjectActor))
  (if _returnvalue
    _
    (else
      (bind _returnvalue_2 (Actor|GetActorOfClass 0 ObjectActor))
      (Utilities|Map|Add (LocalVariables|GetObject%20Class) ObjectActor _returnvalue_2)))
  (return _value))

(fn CreateWidget)

(fn TimeLineLerped)