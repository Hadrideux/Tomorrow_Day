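; Interactable large drawer furniture that slides open and closed on alternate interactions, with a sound for each direction.
; BeginPlay caches the starting relative location of LargeDrawerUp and sets the widget's visibility from IsVisible.
; Interact drives a FlipFlop that plays or reverses a Timeline, offsetting the drawer from its start by the track value times Multiplier, with sweep.
; A DoOnce, reset when the Timeline finishes, blocks re-triggering mid-motion.
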(event EventBeginPlay
  (Utilities|FlowControl|Sequence
    (:then_0
      (Variables|Default|SetStartPos (Variables|/Script/Engine.SceneComponent|GetRelativeLocation (Variables|Default|GetLargeDrawerUp))))
    (:then_1
      (Rendering|SetVisibility (Variables|Default|GetWidget) (Variables|Default|GetIs%20Visible) false))))

(event EventInteract
  (bind _largedrawer (Variables|Default|GetLargeDrawer))
  (bind _returnvalue (Transformation|GetWorldLocation _largedrawer))
  (Utilities|FlowControl|Sequence
    (:then_0
      (Utilities|FlowControl|DoOnce false :!label _label
        (:Completed
          (Utilities|FlowControl|FlipFlop
            (:A
              (Audio|PlaySoundatLocation "/Game/Asset/Sound/Drawer/SW_Drawer_On.SW_Drawer_On" _returnvalue "0, 0, 0" 1.0 1.0 0.0 0 0 0 0)
              (bind _newtrack_1 (Timeline|Timeline Play)
                (:Update
                  (Transformation|SetRelativeLocation (Variables|Default|GetLargeDrawerUp) (+ (* _newtrack_1 (Variables|Default|GetMultiplier)) (Variables|Default|GetStartPos)) true false))
                (:Finished
                  (goto _label Reset))))
            (:B
              (Audio|PlaySoundatLocation "/Game/Asset/Sound/Drawer/SW_Drawer_Off.SW_Drawer_Off" _returnvalue "0, 0, 0" 1.0 1.0 0.0 0 0 0 0)
              (Timeline|Timeline Reverse))))))))

(fn ConstructionScript)