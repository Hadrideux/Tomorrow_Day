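; Interactable washing machine that the player relocates once to a preset MovingSpot actor by holding interact.
; Box overlap shows a widget that turns toward the player each tick; hiding is bound to the Widget component's own end overlap, not the Box's.
; Interact feeds the controller's held time into the widget's progress and teleports the machine past one second.
; After a successful move, Tick keeps the widget hidden.
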(event OnComponentBeginOverlap(Box)
  (params (OverlappedComponent :type Primitive%20Component%20Object%20Reference) (OtherActor :type Actor%20Object%20Reference) (OtherComp :type Primitive%20Component%20Object%20Reference) (OtherBodyIndex :type Integer) (bFromSweep :type Boolean) (SweepResult :type Hit%20Result%20Structure%20%28by%20ref%29))
  ;[1 1 1] Display UI Interact
  (bind _output_get (Variables|Default|SetIs%20Visible true))
  (Rendering|SetVisibility (Variables|Default|GetWidget) _output_get false))

(event OnComponentEndOverlap(Widget)
  (params (OverlappedComponent :type Primitive%20Component%20Object%20Reference) (OtherActor :type Actor%20Object%20Reference) (OtherComp :type Primitive%20Component%20Object%20Reference) (OtherBodyIndex :type Integer))
  ;[1 1 1] Display UI Interact
  (bind _output_get (Variables|Default|SetIs%20Visible false))
  (Rendering|SetVisibility (Variables|Default|GetWidget) _output_get false))

(event Custom|MovingToSpot
  ;[1 1 1] Move To Spot Actor
  (if (not (Variables|Default|GetIsAlreadyMove))
    (bind _returnvalue (Transformation|SetActorLocation (Transformation|GetActorLocation (Variables|Default|GetMovingSpot)) false false))
    (Variables|Default|SetIsAlreadyMove _returnvalue)))

(event Custom|RotationUI
  ;[1 1 1] Target Rotation UI To Character
  (Transformation|SetWorldRotation (Variables|Default|GetWidget) (Math|Rotator|FindLookatRotation (Transformation|GetActorLocation self) (- (Transformation|GetActorLocation (Game|GetPlayerCharacter 0)) "0.000000,0.000000,68.150000")) false false))

(event EventBeginPlay
  (Rendering|SetVisibility (Variables|Default|GetWidget) (Variables|Default|GetIs%20Visible) false)
  (bind _asw_interaction_environnement (Utilities|Casting|CastToW_InteractionEnvironnement (UserInterface|GetWidget (Variables|Default|GetWidget))))
  (Variables|Default|SetWInteraction _asw_interaction_environnement))

(event EventInteract
  (bind _asbp_player_character_controller (Utilities|Casting|CastToBP_PlayerCharacterController (CallFunction|GetUniqueInstance "/Game/Blueprint/Character/BP_PlayerCharacterController.BP_PlayerCharacterController_C")))
  (Default|SetPercent (Variables|Default|GetWInteraction) (Variables|/Game/Blueprint/Character/BP_PlayerCharacterController.BP_PlayerCharacterController_C|GetTriggered%20Seconds _asbp_player_character_controller))
  (if (> (Variables|/Game/Blueprint/Character/BP_PlayerCharacterController.BP_PlayerCharacterController_C|GetTriggered%20Seconds _asbp_player_character_controller) 1.0)
    (CallFunction|MovingtoSpot)))

(event EventTick
  (params (DeltaSeconds :type Float%20%28single-precision%29))
  (Utilities|FlowControl|Sequence
    (:then_0
      (if (Variables|Default|GetIs%20Visible)
        (CallFunction|RotationUI)))
    (:then_1
      (if (Variables|Default|GetIsAlreadyMove)
        (Rendering|SetVisibility (Variables|Default|GetWidget) false false)))))

(fn ConstructionScript)