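; Interactable door that alternately swings open and closed with sound on each interaction.
; Interact passes a DoOnce, reset when the Timeline finishes, into a FlipFlop that plays or reverses the Timeline, adding multiplier-scaled yaw to the starting rotation.
; A prompt widget shows on Box begin overlap, hides on the widget's own end overlap, and RotationUI turns it toward the player.
; DisplayInteraction adds or removes that widget in the viewport based on interface support.
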(event OnComponentBeginOverlap(Box)
  (params (OverlappedComponent :type Primitive%20Component%20Object%20Reference) (OtherActor :type Actor%20Object%20Reference) (OtherComp :type Primitive%20Component%20Object%20Reference) (OtherBodyIndex :type Integer) (bFromSweep :type Boolean) (SweepResult :type Hit%20Result%20Structure%20%28by%20ref%29))
  ;[1 1 1] Display UI Interact
  (bind _output_get (Variables|Default|SetIs%20Visible true))
  (Rendering|SetVisibility (Variables|Default|GetWidget) _output_get false))

(event OnComponentEndOverlap(Widget)
  (params (OverlappedComponent :type Primitive%20Component%20Object%20Reference) (OtherActor :type Actor%20Object%20Reference) (OtherComp :type Primitive%20Component%20Object%20Reference) (OtherBodyIndex :type Integer))
  ;[1 1 1] Display UI Interact
  (bind _output_get (Variables|Default|SetIs%20Visible false))
  (Rendering|SetVisibility (Variables|Default|GetWidget) _output_get false))

(event Custom|RotationUI
  ;[1 1 1] Target Rotation UI To Character
  (Transformation|SetWorldRotation (Variables|Default|GetWidget) (Math|Rotator|FindLookatRotation (Transformation|GetActorLocation self) (- (Transformation|GetActorLocation (Game|GetPlayerCharacter 0)) "0.000000,0.000000,68.150000")) false false))

(event EventBeginPlay
  (Utilities|FlowControl|Sequence
    (:then_0
      (Variables|Default|SetSetRotation (Variables|/Script/Engine.SceneComponent|GetRelativeRotation (Variables|Default|GetDoor))))
    (:then_1
      (Rendering|SetVisibility (Variables|Default|GetWidget) (Variables|Default|GetIs%20Visible) false))))

(event EventInteract
  (bind _door (Variables|Default|GetDoor))
  (bind _returnvalue (Transformation|GetWorldLocation _door))
  (Utilities|FlowControl|DoOnce false :!label _label
    (:Completed
      (Utilities|FlowControl|FlipFlop
        (:A
          (Audio|PlaySoundatLocation "/Game/Asset/Sound/Door/Door_Open.Door_Open" _returnvalue "0, 0, 0" 1.0 1.0 0.0 0 0 0 0)
          (bind _rotation (Timeline|Timeline Play)
            (:Update
              (Transformation|SetRelativeRotation (Variables|Default|GetDoor) (Math|Rotator|MakeRotator 0.0 0.0 (+ (.z (* _rotation (Variables|Default|GetMultiplier))) (.yaw (Variables|Default|GetSetRotation)))) false false))
            (:Finished
              (goto _label Reset))))
        (:B
          (Audio|PlaySoundatLocation "/Game/Asset/Sound/Door/Door_Close.Door_Close" _returnvalue "0, 0, 0" 1.0 1.0 0.0 0 0 0 0)
          (Timeline|Timeline Reverse))))))

(fn ConstructionScript)

(fn DisplayInteraction
  (bind _widget (Variables|Default|GetWidget))
  (bind _returnvalue (UserInterface|GetWidget _widget))
  (bind _returnvalue_2 (UserInterface|Viewport|IsinViewport _returnvalue))
  (if (Utilities|DoesObjectImplementInterface self "/Game/Blueprint/Character/BP_InteractInterface.BP_InteractInterface_C")
    (if (not _returnvalue_2)
      (UserInterface|Viewport|AddtoViewport _returnvalue 0))
    (elif _returnvalue_2
      (Default|RemoveInteraction (.AsW%20Interaction%20Environnement (Utilities|Casting|CastToW_InteractionEnvironnement _returnvalue))))))