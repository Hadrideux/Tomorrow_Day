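; Test actor in the CCTV CameraLive folder that jumps back and forth between two reference points.
; From BeginPlay, a Move event uses a FlipFlop to alternately snap the actor, without sweep, to the locations of the first two actors in its Point array.
; Move calls itself again after a two-second Delay, forming an endless timed loop without Tick.
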(event Custom|Move
  (bind _point (Variables|Default|GetPoint))
  (Utilities|FlowControl|FlipFlop
    (:A
      (Transformation|SetActorLocation (Transformation|GetActorLocation (Utilities|Array|Get(acopy) _point)) false false))
    (:B
      (Transformation|SetActorLocation (Transformation|GetActorLocation (Utilities|Array|Get(acopy) _point 1)) false false)))
  (Utilities|FlowControl|Delay 2.0)
  (CallFunction|Move))

(event EventBeginPlay
  (CallFunction|Move))

(event Collision|EventActorBeginOverlap
  (params (OtherActor :type Actor%20Object%20Reference)))

(fn ConstructionScript)