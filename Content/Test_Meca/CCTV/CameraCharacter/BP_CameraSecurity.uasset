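; BP_CameraSecurity is a test security camera that the player controls through Enhanced Input, with interaction and vision-filter actions.
; The interaction action line-traces on the Visibility channel from the camera along its forward vector up to Range, draws the trace, and prints the hit actor's name.
; The filter action uses a FlipFlop to swap the camera's post-process settings between normal and thermal vision presets.
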(event Input|EnhancedActionEvents|EnhancedInputActionIA_Interaction
  (params (ActionValue :type Boolean) (ElapsedSeconds :type Float%20%28double-precision%29) (TriggeredSeconds :type Float%20%28double-precision%29) (InputAction :type Input%20Action%20Object%20Reference :default "/Game/Test_Meca/CCTV/CameraCharacter/Input/Action/IA_Interaction.IA_Interaction"))
  (bind _camera (Variables|Default|GetCamera))
  (bind _returnvalue (Transformation|GetWorldLocation _camera))
  (:Started
    (bind _outhit (Collision|LineTraceByChannel _returnvalue (+ _returnvalue (* (Math|Vector|GetForwardVector _camera) (Variables|Default|GetRange))) "TraceTypeQuery1" false 0 "ForDuration" true "(R=1.000000,G=0.000000,B=0.000000,A=1.000000)" "(R=0.000000,G=1.000000,B=0.000000,A=1.000000)" 1e+01))
    (Development|PrintString (Utilities|GetDisplayName (.HitActor (Collision|BreakHitResult _outhit))))))

(event Input|EnhancedActionEvents|EnhancedInputActionIA_ChangeFilter
  (params (ActionValue :type Boolean) (ElapsedSeconds :type Float%20%28double-precision%29) (TriggeredSeconds :type Float%20%28double-precision%29) (InputAction :type Input%20Action%20Object%20Reference :default "/Game/Test_Meca/CCTV/CameraCharacter/Input/Action/IA_ChangeFilter.IA_ChangeFilter"))
  (bind _camera (Variables|Default|GetCamera))
  (:Started
    (Utilities|FlowControl|FlipFlop
      (:A
        (Variables|/Script/Engine.CameraComponent|SetPostProcessSettings _camera (Variables|Default|GetNormalVision_PP)))
      (:B
        (Variables|/Script/Engine.CameraComponent|SetPostProcessSettings _camera (Variables|Default|GetThermalVision_PP))))))

(fn ConstructionScript)