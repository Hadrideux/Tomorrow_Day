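; Player controller for TomorrowsDay that relays input and creates the game's UI widgets.
; On BeginPlay it adds the default character mapping context, shows the mouse cursor and creates the hub, registration and cork board screens plus the camera interface.
; Only the camera interface is added to the viewport at start.
; Enhanced Input look and selection actions are rebroadcast through the OnLookAround and OnSelection event dispatchers.
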(event Input|EnhancedActionEvents|EnhancedInputActionIA_Look
  (params (ActionValue :type Vector%202D%20Structure) (ElapsedSeconds :type Float%20%28double-precision%29) (TriggeredSeconds :type Float%20%28double-precision%29) (InputAction :type Input%20Action%20Object%20Reference :default "/Game/Blueprint/Character/Input/Action/Game/IA_Look.IA_Look"))
  (Default|CallOnLookAround ActionValue))

(event Input|EnhancedActionEvents|EnhancedInputActionIA_Selection
  (params (ActionValue :type Boolean) (ElapsedSeconds :type Float%20%28double-precision%29) (TriggeredSeconds :type Float%20%28double-precision%29) (InputAction :type Input%20Action%20Object%20Reference :default "/Game/Blueprint/Character/Input/Action/Game/IA_Selection.IA_Selection"))
  (:Started
    (Default|CallOnSelection)))

(event EventBeginPlay
  (Input|AddMappingContext (PlayerController|LocalPlayerSubsystems|GetEnhancedInputLocalPlayerSubsystem) "/Game/Blueprint/Character/Input/IMC_CharacterDefault.IMC_CharacterDefault" 0 "(bIgnoreAllPressedKeysUntilRelease=True,bForceImmediately=False,bNotifyUserSettings=False)")
  (CallFunction|InitializeCreatingWidget)
  (Variables|Default|SetbShowMouseCursor true))

(fn ConstructionScript)

(fn InitializeCreatingWidget
  (Utilities|FlowControl|Sequence
    (:then_0
      ;[1 1 1] Main Interface
      (bind _returnvalue (UserInterface|CreateWidget "/Game/Widget/HUBScreen/WBP_HUBScreen.WBP_HUBScreen_C"))
      (Variables|Default|SetHUBScreen _returnvalue)
      (bind _returnvalue_2 (UserInterface|CreateWidget "/Game/Widget/RegisScreen/WBP_RegisInterface.WBP_RegisInterface_C"))
      (Variables|Default|SetRegisScreen _returnvalue_2)
      (bind _returnvalue_3 (UserInterface|CreateWidget "/Game/Widget/CorkBoard/WBP_CorkBoardHUD.WBP_CorkBoardHUD_C"))
      (Variables|Default|SetCorkBoard _returnvalue_3))
    (:then_1
      ;[1 1 1] Camera Interface
      (bind _returnvalue_4 (UserInterface|CreateWidget "/Game/Widget/Camera/WBP_CameraInterface.WBP_CameraInterface_C"))
      (bind _output_get (Variables|Default|SetCameraInterface _returnvalue_4))
      (UserInterface|Viewport|AddtoViewport _output_get 0))))