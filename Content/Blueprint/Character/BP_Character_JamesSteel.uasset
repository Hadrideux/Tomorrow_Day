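; James Steel character that looks around within a limited view, zooms and interacts with what the camera faces.
; Look and selection come from player controller dispatchers, while zoom input plays and reverses a timeline that narrows camera FOV.
; Selection line-traces from the camera, asking the controller to possess a hit pawn or starting a new investigation on a fax.
; Camera manager pitch and yaw limits are centred on camera rotation, set at construction and BeginPlay.
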(event Custom|OnLookAround
  (params (ActionValue :type Vector%202D%20Structure))
  (CallFunction|LookAround ActionValue))

(event Custom|BindLookAround
  (EventDispatchers|AssignOnLookAround (Variables|Default|GetPlayerController) (delegate Custom|OnLookAround)))

(event Custom|BindSelection
  (EventDispatchers|AssignOnSelection (Variables|Default|GetPlayerController) (delegate Custom|OnSelection)))

(event Custom|OnSelection
  (bind _hitactor (CallFunction|ObjectClicked))
  (bind _aspawn (Utilities|Casting|CastToPawn _hitactor)
    (:then
      (Default|CallOnNewPossessPawn (Variables|Default|GetPlayerController) _aspawn))
    (:CastFailed
      (bind _asbp_fax (Utilities|Casting|CastToBP_Fax _hitactor))
      (Default|StartNewInvestigation _asbp_fax))))

(event Input|EnhancedActionEvents|EnhancedInputActionIA_Zoom
  (params (ActionValue :type Boolean) (ElapsedSeconds :type Float%20%28double-precision%29) (TriggeredSeconds :type Float%20%28double-precision%29) (InputAction :type Input%20Action%20Object%20Reference :default "/Game/Blueprint/Character/Input/Action/Game/IA_Zoom.IA_Zoom"))
  (:Started
    (bind _zoom (Timeline|Zoom Play)
      (:Update
        (Camera|SetFieldOfView (Variables|Default|GetCamera) (Math|Float|Lerp 9e+01 45.0 _zoom)))))
  (:Completed
    (Timeline|Zoom Reverse)))

(event EventBeginPlay
  (Utilities|FlowControl|Sequence
    (:then_0
      (bind _asbp_tomorrows_day_pc (Utilities|Casting|CastToBP_TomorrowsDay_PC (Game|GetPlayerController 0)))
      (Variables|Default|SetPlayerController _asbp_tomorrows_day_pc)
      (CallFunction|BindLookAround)
      (CallFunction|BindSelection))
    (:then_1
      (bind _asbp_scene_manager (Utilities|Casting|CastToBP_SceneManager (CallFunction|GetSingletonInstance "/Game/Blueprint/Global/Manager/BP_SceneManager.BP_SceneManager_C")))
      (Variables|Default|SetScene%20Manager _asbp_scene_manager)
      (CallFunction|Contraint))))

(fn ConstructionScript
  (CallFunction|Contraint))

(fn LookAround
  (params (InputAxis :type Vector%202D%20Structure))
  (Pawn|Input|AddControllerYawInput (.x InputAxis))
  (Pawn|Input|AddControllerPitchInput (.y InputAxis)))

(fn Contraint
  (bind _returnvalue (Game|GetPlayerCameraManager 0))
  (bind _camera (Variables|Default|GetCamera))
  (bind _returnvalue_2 (Transformation|GetWorldRotation _camera))
  (Utilities|FlowControl|Sequence
    (:then_0
      (Variables|/Script/Engine.PlayerCameraManager|SetViewPitchMax _returnvalue (+ (Variables|ContraintView|GetPitchValue) (.pitch _returnvalue_2)))
      (Variables|/Script/Engine.PlayerCameraManager|SetViewYawMax _returnvalue (+ (Variables|ContraintView|GetYawValue) (.yaw _returnvalue_2))))
    (:then_1
      (Variables|/Script/Engine.PlayerCameraManager|SetViewPitchMin _returnvalue (- (.pitch _returnvalue_2) (Variables|ContraintView|GetPitchValue)))
      (Variables|/Script/Engine.PlayerCameraManager|SetViewYawMin _returnvalue (- (.yaw _returnvalue_2) (Variables|ContraintView|GetYawValue))))))

(fn ObjectClicked
  (bind _camera (Variables|Default|GetCamera))
  (bind _returnvalue (Transformation|GetWorldLocation _camera))
  (bind _outhit (Collision|LineTraceByChannel _returnvalue (+ _returnvalue (* (Math|Vector|GetForwardVector (Transformation|GetWorldRotation (Variables|Default|GetCamera))) 1e+03)) "TraceTypeQuery3" true 0 "ForDuration"))
  (return (.HitActor (Collision|BreakHitResult _outhit))))