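; BP_SequencerController drives the penthouse level sequence in response to events from BP_SequencerManager.
; One second after BeginPlay, it fetches the manager singleton and binds to its time-code and play/pause events.
; Time-code changes call PlayTo on the manager's sequence at the incoming value scaled by a hardcoded 160-second factor, and play/pause events play or pause that sequence.
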(event Custom|BindSequencerTime
  ;[0.2672 1 0.1234] TimeCode Sequence
  (EventDispatchers|BindEventtoOnChangeTimeCode (Variables|Default|GetSequencerManager) (delegate Custom|OnChangeTimeCcode)))

(event Custom|OnChangeTimeCcode
  (params (SequencerTime :type Float%20%28double-precision%29))
  ;[0.2672 1 0.1234] TimeCode Sequence
  (Class|MovieSceneSequencePlayer|Playto (Variables|/Game/Blueprint/Global/Manager/BP_SequencerManager.BP_SequencerManager_C|GetPentHouseSequene (Variables|Default|GetSequencerManager)) (Utilities|Struct|MakeMovieSceneSequencePlaybackParams "(FrameNumber=(Value=0),SubFrame=0.000000)" (* SequencerTime 1.6e+02) "" "Time" "Play" false)))

(event Custom|OnPlaySequence
  (params (Play/Pause :type EPlaySequence%20Enum :default "NewEnumerator0"))
  (bind _sequencermanager (Variables|Default|GetSequencerManager))
  (bind _penthousesequene (Variables|/Game/Blueprint/Global/Manager/BP_SequencerManager.BP_SequencerManager_C|GetPentHouseSequene _sequencermanager))
  ;[1 0.1311 0.07812] Play/Pause Sequence
  (switch Utilities|FlowControl|Switch|SwitchonEPlaySequence Play/Pause
    (:NewEnumerator1
      (Sequencer|Player|Play _penthousesequene :!class /Script/MovieScene.MovieSceneSequencePlayer))
    (:NewEnumerator2
      (Sequencer|Player|Pause _penthousesequene))))

(event Custom|BindPlaySequence
  ;[1 0.1311 0.07812] Play/Pause Sequence
  (EventDispatchers|BindEventtoOnPlaySequence (Variables|Default|GetSequencerManager) (delegate Custom|OnPlaySequence)))

(event EventBeginPlay
  (Utilities|FlowControl|Delay 1.0)
  (Variables|Default|SetSequencerManager (.AsBP%20Sequencer%20Manager (Utilities|Casting|CastToBP_SequencerManager (CallFunction|GetSingletonInstance "/Game/Blueprint/Global/Manager/BP_SequencerManager.BP_SequencerManager_C"))))
  (CallFunction|BindAllEvent))

(fn ConstructionScript)

(fn BindAllEvent
  (CallFunction|BindSequencerTime)
  (CallFunction|BindPlaySequence))