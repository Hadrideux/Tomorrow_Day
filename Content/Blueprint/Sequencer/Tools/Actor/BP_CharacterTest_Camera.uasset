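; Test camera actor for sequencer tooling that rides along the spline of an assigned pathing object.
; On BeginPlay it snaps to its stored spline distance if a path is valid.
; IncreasedPathing scales a timeline value by spline length, clamps it and repositions the actor, without a validity check.
; Placement teleports the actor to the spline's world location and rotation at that distance.
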(event EventBeginPlay
  (CallFunction|Pathing))

(fn ConstructionScript)

(fn Pathing
  (Utilities|IsValid (Variables|Default|GetCurrentPathing)
    (:Is%20Valid
      (CallFunction|PlaceinPathing))))

(fn IncreasedPathing
  (params (NewTimeLine :type Float%20%28double-precision%29))
  (bind _currentpathing (Variables|Default|GetCurrentPathing))
  (bind _spline (Variables|/Game/ProtoMeca_2/Hint/BP_PathingTest.BP_PathingTest_C|GetSpline _currentpathing))
  (bind _returnvalue (Spline|GetSplineLength _spline))
  (Variables|Default|SetSplineDistance (Math|Float|Clamp(Float) (* NewTimeLine _returnvalue) 0.0 _returnvalue))
  (CallFunction|PlaceinPathing))

(fn PlaceinPathing
  (bind _currentpathing (Variables|Default|GetCurrentPathing))
  (bind _splinedistance (Variables|Default|GetSplineDistance))
  (bind _spline (Variables|/Game/ProtoMeca_2/Hint/BP_PathingTest.BP_PathingTest_C|GetSpline _currentpathing))
  (bind _returnvalue (Spline|GetTransformatDistanceAlongSpline _spline _splinedistance "World" false))
  (Transformation|SetActorLocation (.location _returnvalue) false true)
  (Transformation|SetActorRotation (.rotation _returnvalue) true))