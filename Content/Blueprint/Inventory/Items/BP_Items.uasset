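; BP_Items is a world item pickup that transfers its ItemObject into a character's inventory on touch.
; On BeginPlay it fills a missing ItemObject from GetDefautItemObject, which returns nothing here and appears intended for child overrides.
; When its Box overlaps a BP_CharacterController actor, it calls TryAddItem on that actor's BPInventoryComponent and destroys itself only if the add succeeds.
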(event OnComponentBeginOverlap(Box)
  (params (OverlappedComponent :type Primitive%20Component%20Object%20Reference) (OtherActor :type Actor%20Object%20Reference) (OtherComp :type Primitive%20Component%20Object%20Reference) (OtherBodyIndex :type Integer) (bFromSweep :type Boolean) (SweepResult :type Hit%20Result%20Structure%20%28by%20ref%29))
  (bind _asbp_character_controller (Utilities|Casting|CastToBP_CharacterController OtherActor))
  (bind _added (Default|TryAddItem (Variables|/Game/Blueprint/Character/BP_CharacterController.BP_CharacterController_C|GetBP_InventoryComponent _asbp_character_controller) (Variables|Private|GetItemObject)))
  (if _added
    (Actor|DestroyActor)))

(event EventBeginPlay
  (if (not (Utilities|IsValid (Variables|Private|GetItemObject)))
    (bind _itemoject (Public|GetDefautItemObject))
    (Variables|Private|SetItemObject _itemoject)))

(fn ConstructionScript)

(fn GetDefautItemObject
  (return 0))