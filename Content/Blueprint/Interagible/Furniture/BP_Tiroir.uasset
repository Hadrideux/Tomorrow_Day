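; Interactable furniture drawer that slides open and closed when Interact fires.
; A Timeline offsets the Tiroir component from its starting position with a swept move, playing or reversing based on IsOpened, which flips on every Update.
; Box begin overlap shows the prompt widget and Widget end overlap hides it; while visible, Tick turns it toward the player character.
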(event OnComponentBeginOverlap(Box)
  (params (OverlappedComponent :type Primitive%20Component%20Object%20Reference) (OtherActor :type Actor%20Object%20Reference) (OtherComp :type Primitive%20Component%20Object%20Reference) (OtherBodyIndex :type Integer) (bFromSweep :type Boolean) (SweepResult :type Hit%20Result%20Structure%20%28by%20ref%29))
  ;[1 1 1] Display UI Interact
  (bind _output_get (Variables|Default|SetIs%20Visible true))
  (Rendering|SetVisibility (Variables|Default|GetWidget) _output_get false))

(event OnComponentEndOverlap(Widget)
  (params (OverlappedComponent :type Primitive%20Component%20Object%20Reference) (OtherActor :type Actor%20Object%20Reference) (OtherComp :type Primitive%20Component%20Object%20Reference) (OtherBodyIndex :type Integer))
  ;[1 1 1] Display UI Interact
  (bind _output_get (Variables|Default|SetIs%20Visible false))
  (Rendering|SetVisibility (Variables|Default|GetWidget) _output_get false))

(event Custom|RotationUI
  ;[1 1 1] Target Rotation UI To Character
  (Transformation|SetWorldRotation (Variables|Default|GetWidget) (Math|Rotator|FindLookatRotation (Transformation|GetActorLocation self) (- (Transformation|GetActorLocation (Game|GetPlayerCharacter 0)) "0.000000,0.000000,68.150000")) false false))

(event EventInteract
  (if (Variables|Default|GetIsOpened)
    (bind _newtrack_1 (Timeline|Timeline Reverse)
      (:Update
        (Transformation|SetRelativeLocation (Variables|Default|GetTiroir) (+ _newtrack_1 (Variables|Default|GetPos1)) true false)
        (Variables|Default|SetIsOpened (not (Variables|Default|GetIsOpened)))))
    (else
      (Timeline|Timeline Play))))

(event EventTick
  (params (DeltaSeconds :type Float%20%28single-precision%29))
  (if (Variables|Default|GetIs%20Visible)
    (CallFunction|RotationUI)))

(event EventBeginPlay
  (Utilities|FlowControl|Sequence
    (:then_0
      (Variables|Default|SetPos1 (Variables|/Script/Engine.SceneComponent|GetRelativeLocation (Variables|Default|GetTiroir))))
    (:then_1
      (Rendering|SetVisibility (Variables|Default|GetWidget) (Variables|Default|GetIs%20Visible) false))))

(fn ConstructionScript)