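; Interactable drawer furniture that slides open and closed with matching sounds when Interact is called.
; A FlipFlop plays or reverses a Timeline that offsets the drawer mesh from its starting position with sweep, gated by a DoOnce that resets when the Timeline finishes.
; While IsVisible is true, Tick turns the widget toward the player character.
; The logic that toggles widget visibility is unwired, so only BeginPlay applies it.
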(event Custom|RotationUI
  ;[1 1 1] Target Rotation UI To Character
  (Transformation|SetWorldRotation (Variables|Default|GetWidget) (Math|Rotator|FindLookatRotation (Transformation|GetActorLocation self) (- (Transformation|GetActorLocation (Game|GetPlayerCharacter 0)) "0.000000,0.000000,68.150000")) false false))

(event EventInteract
  (bind _meuble_tiroir (Variables|Default|GetMeuble_Tiroir))
  (bind _returnvalue (Transformation|GetWorldLocation _meuble_tiroir))
  (Utilities|FlowControl|DoOnce false :!label _label
    (:Completed
      (Utilities|FlowControl|FlipFlop
        (:A
          (Audio|PlaySoundatLocation "/Game/Asset/Sound/Drawer/SW_Drawer_On.SW_Drawer_On" _returnvalue "0, 0, 0" 1.0 1.0 0.0 0 0 0 0)
          (bind _newtrack_1 (Timeline|Timeline Play)
            (:Update
              (Transformation|SetRelativeLocation (Variables|Default|GetTiroir) (+ (* _newtrack_1 (Variables|Default|GetMultiplier)) (Variables|Default|GetStartPos)) true false))
            (:Finished
              (goto _label Reset))))
        (:B
          (Audio|PlaySoundatLocation "/Game/Asset/Sound/Drawer/SW_Drawer_Off.SW_Drawer_Off" _returnvalue "0, 0, 0" 1.0 1.0 0.0 0 0 0 0)
          (Timeline|Timeline Reverse))))))

(event EventTick
  (params (DeltaSeconds :type Float%20%28single-precision%29))
  (if (Variables|Default|GetIs%20Visible)
    (CallFunction|RotationUI)))

(event EventBeginPlay
  (Utilities|FlowControl|Sequence
    (:then_0
      (Variables|Default|SetStartPos (Variables|/Script/Engine.SceneComponent|GetRelativeLocation (Variables|Default|GetTiroir))))
    (:then_1
      (Rendering|SetVisibility (Variables|Default|GetWidget) (Variables|Default|GetIs%20Visible) false))))

(fn ConstructionScript)