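; Interactable resource actor that spawns as a random resource and shows an interaction prompt with its name when approached.
; On BeginPlay it picks a random DataRessource table row, applies that row's mesh and a random rotation, and stores the row name as display name.
; Box overlap toggles the W_InteractionEnvironnement widget, which rotates each tick to face the player while visible.
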(event OnComponentBeginOverlap(Box)
  (params (OverlappedComponent :type Primitive%20Component%20Object%20Reference) (OtherActor :type Actor%20Object%20Reference) (OtherComp :type Primitive%20Component%20Object%20Reference) (OtherBodyIndex :type Integer) (bFromSweep :type Boolean) (SweepResult :type Hit%20Result%20Structure%20%28by%20ref%29))
  ;[1 1 1] Display UI Interact
  (bind _output_get (Variables|UI|SetIsVisible true))
  (CallFunction|DisplayWidgetInteraction _output_get (Variables|UI|GetDisplayName)))

(event OnComponentEndOverlap(Box)
  (params (OverlappedComponent :type Primitive%20Component%20Object%20Reference) (OtherActor :type Actor%20Object%20Reference) (OtherComp :type Primitive%20Component%20Object%20Reference) (OtherBodyIndex :type Integer))
  ;[1 1 1] Display UI Interact
  (bind _output_get (Variables|UI|SetIsVisible false))
  (CallFunction|DisplayWidgetInteraction _output_get "None"))

(event Custom|RotationUI
  ;[1 1 1] Target Rotation UI To Character
  (if (Variables|UI|GetIsVisible)
    (Transformation|SetWorldRotation (Variables|Default|GetWidget) (Math|Rotator|FindLookatRotation (Transformation|GetActorLocation self) (Transformation|GetActorLocation (Game|GetPlayerCharacter 0))) false false)))

(event EventBeginPlay
  (Utilities|FlowControl|Sequence
    (:then_0
      (bind _out_row (CallFunction|GetDataRessource self))
      (Components|StaticMesh|SetStaticMesh (Variables|Default|GetModel) (.Mesh (Utilities|Struct|BreakS_Ressource _out_row))))
    (:then_1
      (Transformation|SetRelativeRotation (Variables|Default|GetModel) (Math|Random|RandomRotator false) false false))
    (:then_2
      (CallFunction|DisplayWidgetInteraction (Variables|UI|GetIsVisible) "None"))))

(event EventTick
  (params (DeltaSeconds :type Float%20%28single-precision%29))
  (if (Variables|UI|GetIsVisible)
    (CallFunction|RotationUI)))

(fn ConstructionScript)

(fn GetDataRessource
  (bind _dataressource (Variables|Data|GetDataRessource))
  (bind _outrownames (DataTable|GetDataTableRowNames _dataressource))
  (bind _output_get (Variables|Data|SetData%20RowHandle (Utilities|Struct|MakeDataTableRowHandle _dataressource (.OutItem (Utilities|Array|Random _outrownames)))))
  (bind _output_get_2 (Variables|UI|SetDisplayName (.rowname _output_get)))
  (bind _returnvalue (Utilities|GetDataTableRow (.datatable _output_get) _output_get_2)
    (:then
      (return _returnvalue))))

(fn DisplayWidgetInteraction
  (params (IsVisible :type Boolean) (ObjectName :type Name))
  (bind _widget (Variables|Default|GetWidget))
  (Rendering|SetVisibility _widget IsVisible false)
  (bind _asw_interaction_environnement (Utilities|Casting|CastToW_InteractionEnvironnement (UserInterface|GetUserWidgetObject _widget)))
  (Rendering|Components|TextRender|SetText (Variables|/Game/Blueprint/UI_Blueprint/InGame/W_InteractionEnvironnement.W_InteractionEnvironnement_C|GetObjectName _asw_interaction_environnement) (Utilities|Text|ToText(Name) ObjectName)))