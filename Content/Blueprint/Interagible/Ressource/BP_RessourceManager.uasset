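; BP_RessourceManager checks which resource type the character is targeting.
; Every Tick, it compares the character's HitActor to BP_RessourceController, casts it and reads its resource data through GetDataRessource.
; A switch on TypeRessource routes to the TargetFood or TargetComponent event, which currently only print the type name.
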(event Custom|TargetFood
  (Development|PrintString "Food" true true "(R=0.000000,G=0.660000,B=1.000000,A=1.000000)" 5.0 "Ressource : "))

(event Custom|TargetComponent
  (Development|PrintString "Component"))

(event EventTick
  (params (DeltaSeconds :type Float%20%28single-precision%29))
  (bind _character (Variables|Default|GetCharacter))
  (bind _hit_actor (Variables|/Game/Blueprint/Character/BP_CharacterController.BP_CharacterController_C|GetHit%20Actor _character))
  (if (== _hit_actor "/Game/Blueprint/Interagible/Ressource/BP_RessourceController.BP_RessourceController")
    (bind _asbp_ressource_controller (Utilities|Casting|CastToBP_RessourceController _hit_actor))
    (bind _out_row (Default|GetDataRessource _asbp_ressource_controller))
    (switch Utilities|FlowControl|Switch|SwitchonE_TypeObject (.typeressource _out_row)
      (:NewEnumerator0
        (CallFunction|TargetFood))
      (:NewEnumerator2
        (CallFunction|TargetComponent)))))

(fn ConstructionScript)