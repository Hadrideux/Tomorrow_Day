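; Investigation camera controller that switches between placed camera positions, changes post-process filters and lets the player pick hints to analyse.
; It registers with the SceneManager's CameraManager and binds to its filter and position events, plus the UIManager's analyse choice.
; Selection line-traces under the cursor for an AC_HintInformation, shows the analyse widget, then START or BREAK drives InvestigationManager analysis requests.
; A SceneCapture2D renders to a render target.
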(event Custom|BindChangeCameraEvent
  ;[1 0.1098 0.0902] Change Camera Position
  (EventDispatchers|BindEventtoOnChangeCameraPosition (Variables|/Game/Blueprint/Global/Manager/BP_SceneManager.BP_SceneManager_C|GetCameraManager (Variables|Manager|GetScene%20Manager)) (delegate Custom|ChangeCameraPosition)))

(event Custom|ChangeCameraPosition
  (params (PositionIndex :type Integer))
  ;[1 0.1098 0.0902] Change Camera Position
  (CameraPosition|SwitchCameraLocation PositionIndex))

(event Custom|BindDurationAnalyseChoice
  ;[1 1 1] Set Analyse
  (EventDispatchers|BindEventtoOnAnalyseChoice (Variables|/Game/Blueprint/Global/Manager/BP_SceneManager.BP_SceneManager_C|GetUIManager (Variables|Manager|GetScene%20Manager)) (delegate Custom|StartAnalyse)))

(event Custom|BindFilterEvent
  ;[0.102 0.2196 1] Filter Change Event
  (EventDispatchers|BindEventtoOnChangeFilter (Variables|/Game/Blueprint/Global/Manager/BP_SceneManager.BP_SceneManager_C|GetCameraManager (Variables|Manager|GetScene%20Manager)) (delegate Custom|ChangeFIlter)))

(event Custom|ChangeFIlter
  (params (SelectedFilter :type ETypeFilter%20Enum :default "NewEnumerator0") (PostProcessIndex :type Integer))
  ;[0.102 0.2196 1] Filter Change Event
  (Default|SetSelectedFilter (Variables|Default|GetAC_CameraFilter) SelectedFilter PostProcessIndex (Variables|/Game/Blueprint/Global/Manager/BP_SceneManager.BP_SceneManager_C|GetCameraManager (Variables|Manager|GetScene%20Manager))))

(event Custom|StartAnalyse
  (params (Analyse%20Choice :type EAnalyseState%20Enum :default "NewEnumerator0"))
  ;[1 1 1] Set Analyse
  (switch Utilities|FlowControl|Switch|SwitchonEAnalyseState Analyse%20Choice
    (:NewEnumerator1
      (HintAnalysis|AddHinttoInvestigation (Variables|Default|GetHintComponent)))
    (:NewEnumerator2
      (Default|CallOnAnalyseRequest (Variables|/Game/Blueprint/Global/Manager/BP_SceneManager.BP_SceneManager_C|GetInvestigation%20Manager (Variables|Manager|GetScene%20Manager)) true))))

(event Input|EnhancedActionEvents|EnhancedInputActionIA_Selection
  (params (ActionValue :type Boolean) (ElapsedSeconds :type Float%20%28double-precision%29) (TriggeredSeconds :type Float%20%28double-precision%29) (InputAction :type Input%20Action%20Object%20Reference :default "/Game/Blueprint/Character/Input/Action/Game/IA_Selection.IA_Selection"))
  ;[1 1 1] Hint Selected
  (:Started
    (bind _hitactor (SelectionHint|MousePositiontoWorldLocation))
    (HintAnalysis|DisplayAnalyseWidget)
    (Utilities|IsValid (Actor|GetComponentbyClass _hitactor "/Game/Blueprint/Hint/AC_HintInformation.AC_HintInformation_C")
      (:Is%20Valid
        (Variables|Default|SetHintComponent (Actor|GetComponentbyClass _hitactor "/Game/Blueprint/Hint/AC_HintInformation.AC_HintInformation_C"))))))

(event EventPossessed
  (params (NewController :type Controller%20Object%20Reference))
  ;[1 1 1] Add Camera Interface On Possess
)

(event EventBeginPlay
  (Utilities|FlowControl|Sequence
    (:then_0
      (bind _asbp_scene_manager (Utilities|Casting|CastToBP_SceneManager (CallFunction|GetSingletonInstance "/Game/Blueprint/Global/Manager/BP_SceneManager.BP_SceneManager_C")))
      (bind _output_get (Variables|Manager|SetScene%20Manager _asbp_scene_manager))
      (Variables|/Game/Blueprint/Global/Manager/BP_CameraManager.BP_CameraManager_C|SetCameraController (Variables|/Game/Blueprint/Global/Manager/BP_SceneManager.BP_SceneManager_C|GetCameraManager _output_get) self))
    (:then_1
      (Event|BindAllEvent))))

(event EventUnpossessed
  (params (OldController :type Controller%20Object%20Reference))
  ;[1 1 1] Add Camera Interface On Possess
)

(fn ConstructionScript
  (Variables|/Script/Engine.SceneCaptureComponent2D|SetTextureTarget (Variables|Default|GetSceneCaptureComponent2D) "/Game/Asset/Texture/CameraView/RT_CameraTest.RT_CameraTest"))

(fn DisplayAnalyseWidget
  (Widget|SetVisibility (Variables|/Game/Widget/Camera/WBP_CameraInterface.WBP_CameraInterface_C|GetWBP_AnalyseInProgress (Variables|/Game/Blueprint/Character/BP_TomorrowsDay_PC.BP_TomorrowsDay_PC_C|GetCameraInterface (.AsBP%20Tomorrows%20Day%20PC (Utilities|Casting|CastToBP_TomorrowsDay_PC (Game|GetPlayerController 0))))) "Visible"))

(fn SwitchCameraLocation
  (params (Position :type Integer))
  (bind _scene_manager (Variables|Manager|GetScene%20Manager))
  (bind _cameramanager (Variables|/Game/Blueprint/Global/Manager/BP_SceneManager.BP_SceneManager_C|GetCameraManager _scene_manager))
  (bind _cameraposition (Variables|/Game/Blueprint/Global/Manager/BP_CameraManager.BP_CameraManager_C|GetCameraPosition _cameramanager))
  (bind _output (Utilities|Array|Get(acopy) _cameraposition Position))
  (Utilities|IsValid _output
    (:Is%20Valid
      (Transformation|SetActorTransform (Transformation|GetActorTransform _output) true))
    (:Is%20Not%20Valid
      (Development|PrintString "Position not found"))))

(fn MousePositiontoWorldLocation
  (bind _returnvalue (Game|GetPlayerController 0))
  (bind (_worldlocation _worlddirection) (Game|Player|ConvertMouseLocationToWorldSpace _returnvalue))
  (bind _outhit (Collision|LineTraceByChannel _worldlocation (+ _worldlocation (* _worlddirection 1e+03)) "TraceTypeQuery1" true 0 "ForDuration"))
  (return (.HitActor (Collision|BreakHitResult _outhit))))

(fn AddHinttoInvestigation
  (params (Hint%20for%20Analyse :type AC%20Hint%20Information%20Object%20Reference))
  (bind _scene_manager (Variables|Manager|GetScene%20Manager))
  (bind _investigation_manager (Variables|/Game/Blueprint/Global/Manager/BP_SceneManager.BP_SceneManager_C|GetInvestigation%20Manager _scene_manager))
  (Utilities|IsValid (Variables|/Game/Blueprint/Global/Manager/BP_InvestigationManager.BP_InvestigationManager_C|GetHint%20for%20Analyse (Variables|/Game/Blueprint/Global/Manager/BP_SceneManager.BP_SceneManager_C|GetInvestigation%20Manager (Variables|Manager|GetScene%20Manager)))
    (:Is%20Valid
      (Development|PrintString "Analysis already in progress"))
    (:Is%20Not%20Valid
      (Variables|/Game/Blueprint/Global/Manager/BP_InvestigationManager.BP_InvestigationManager_C|SetHint%20for%20Analyse _investigation_manager Hint%20for%20Analyse)
      (Default|CallOnAnalyseRequest _investigation_manager false))))

(fn BindAllEvent
  (CallFunction|BindFilterEvent)
  (CallFunction|BindChangeCameraEvent)
  (CallFunction|BindDurationAnalyseChoice))