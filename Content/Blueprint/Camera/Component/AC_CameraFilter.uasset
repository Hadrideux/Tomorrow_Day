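; Camera component that handles vision filters (audio, thermal, UV), switching post-process materials and the hint decals tied to each filter.
; GetSelectedFilter picks the matching hint list from the BP_SceneManager singleton's HintManager, hides the last shown decals and reveals the new ones, or only hides on NONE.
; Separately, EnablePostProcess zeroes the cached previous material's blend weight, sets the chosen index to full weight and caches it.
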(fn GetPostProcessMaterial
  (params (CameraManager :type BP%20Camera%20Manager%20Object%20Reference))
  (return (Utilities|Struct|BreakWeightedBlendables (Utilities|Struct|BreakPostProcessSettings (Variables|/Script/Engine.PostProcessVolume|GetSettings (Variables|/Game/Blueprint/Global/Manager/BP_CameraManager.BP_CameraManager_C|GetPostProcessVolume CameraManager))))))

(fn GetSelectedFilter
  (params (GetFilterType :type ETypeFilter%20Enum :default "NewEnumerator0"))
  (bind _output_get (CallFunction|GetSingletonInstance "/Game/Blueprint/Global/Manager/BP_SceneManager.BP_SceneManager_C"))
  (bind _asbp_scene_manager (Utilities|Casting|CastToBP_SceneManager _output_get))
  (bind _hintmanager (Variables|/Game/Blueprint/Global/Manager/BP_SceneManager.BP_SceneManager_C|GetHintManager _asbp_scene_manager))
  (switch Utilities|FlowControl|Switch|SwitchonETypeFilter GetFilterType
    (:NewEnumerator0
      (Filter|DisableHintfromLastFilter (Variables|Default|GetCurrentSelectedHint)))
    (:NewEnumerator1
      (Filter|DisplayHintfromCurrentFilter (Variables|Default|GetCurrentSelectedHint) (Variables|/Game/Blueprint/Global/Manager/BP_HintManager.BP_HintManager_C|GetAudioHint _hintmanager)))
    (:NewEnumerator2
      (Filter|DisplayHintfromCurrentFilter (Variables|Default|GetCurrentSelectedHint) (Variables|/Game/Blueprint/Global/Manager/BP_HintManager.BP_HintManager_C|GetThermalHint _hintmanager)))
    (:NewEnumerator3
      (Filter|DisplayHintfromCurrentFilter (Variables|Default|GetCurrentSelectedHint) (Variables|/Game/Blueprint/Global/Manager/BP_HintManager.BP_HintManager_C|GetUVHint _hintmanager)))))

(fn DisplayHintfromCurrentFilter
  (params (PreviousHint :type Array%20of%20BP%20General%20Hint%20Object%20References) (SelectedHint :type Array%20of%20BP%20General%20Hint%20Object%20References))
  (Utilities|FlowControl|Sequence
    (:then_0
      (Filter|DisableHintfromLastFilter PreviousHint))
    (:then_1
      (Filter|EnableHintfromCurrentFilter SelectedHint)
      (Variables|Default|SetCurrentSelectedHint SelectedHint))))

(fn DisableHintfromLastFilter
  (params (PreviousHint :type Array%20of%20BP%20General%20Hint%20Object%20References))
  (for _array_element PreviousHint
    (Filter|SetVisibilityDecalHint _array_element false))
  (Development|PrintString "Last Hint Hidden"))

(fn EnableHintfromCurrentFilter
  (params (Hint :type Array%20of%20BP%20General%20Hint%20Object%20References))
  (for _array_element Hint
    (Filter|SetVisibilityDecalHint _array_element true))
  (Development|PrintString "Current Hint Visible"))

(fn SetVisibilityDecalHint
  (params (Decal%20Visibility :type BP%20General%20Hint%20Object%20Reference) (bNewVisibility :type Boolean))
  (Rendering|SetVisibility (Variables|/Game/Blueprint/Hint/BP_GeneralHint.BP_GeneralHint_C|GetVisualFilter Decal%20Visibility) bNewVisibility false))

(fn EnablePostProcess
  (params (CameraManager :type BP%20Camera%20Manager%20Object%20Reference) (PostProcessIndex :type Integer))
  (bind _array (PostProcess|GetPostProcessMaterial CameraManager))
  ;[1 1 1] Deactive Previous PostProcess Filter
  (PostProcess|SetPostProcessFilter _array (Utilities|Array|FindItem _array (Variables|Default|GetPreviousFilter)) 0.0)
  ;[1 1 1] Active and Cache Current PostProcess Filter
  (PostProcess|SetPostProcessFilter _array PostProcessIndex 1.0)
  (Variables|Default|SetPreviousFilter (Utilities|Array|Get(acopy) _array PostProcessIndex)))

(fn SetPostProcessFilter
  (params (PostProcess :type Array%20of%20Weighted%20Blendable%20Structures) (PostProcessIndex :type Integer) (PostProcessWeight :type Float%20%28single-precision%29))
  (Utilities|Array|SetArrayElem PostProcess PostProcessIndex (Utilities|Struct|MakeWeightedBlendable PostProcessWeight (.object (Utilities|Array|Get(acopy) PostProcess PostProcessIndex)))))