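; BP_HUBScreen connects the investigation game's managers to the office HUB screen widgets held by the player controller.
; Once the SceneManager singleton initializes, it caches the Investigation, Data and Camera managers and binds their events.
; These feed the analysis report, citizen search results and map suspect, and show a timed popup on archive selection.
; The pin button displays the suspect's map ping and reveals a hard-coded Amy Powels element on the corkboard.
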(event Custom|CustomEvent
  (Class|MenuAnchor|Close (Variables|/Game/Widget/HUBScreen/WBP_HUBScreen.WBP_HUBScreen_C|GetPopup (Variables|/Game/Blueprint/Global/BP_TomorrowsDay_PC.BP_TomorrowsDay_PC_C|GetHUBScreen (Variables|Manager|GetTomorrows%20Day%20PC)))))

(event Custom|BindingInitiate_Event
  ;[1 1 1] Initialization Binding Event
  (Utilities|FlowControl|Sequence
    (:then_0
      (Initialization|SetManagerVariable))
    (:then_1
      (Initialization|BindAllEvent)
      (bind _returnvalue (UserInterface|CreateWidget "/Game/Widget/Notifications/WBP_ArchivedOpen.WBP_ArchivedOpen_C"))
      (Variables|/Game/Widget/HUBScreen/WBP_HUBScreen.WBP_HUBScreen_C|SetArchivedOpen (Variables|/Game/Blueprint/Global/BP_TomorrowsDay_PC.BP_TomorrowsDay_PC_C|GetHUBScreen (Variables|Manager|GetTomorrows%20Day%20PC)) _returnvalue))))

(event Custom|BindInit
  ;[1 1 1] Initialization Binding Event
  (bind _output_get (Variables|Manager|SetScene%20Manager (.AsBP%20Scene%20Manager (Utilities|Casting|CastToBP_SceneManager (CallFunction|GetSingletonInstance "/Game/Blueprint/Global/Manager/BP_SceneManager.BP_SceneManager_C")))))
  (EventDispatchers|AssignOnInitializationBind _output_get (delegate Custom|BindingInitiate_Event)))

(event Custom|BindArchiveSelected
  (EventDispatchers|BindEventtoOnArchiveSelected (Variables|Default|GetCamera%20Manager) (delegate Custom|ArchiveSelected_Event)))

(event Custom|ArchiveSelected_Event
  (params (bIsSelected :type Boolean))
  (Class|MenuAnchor|Open (Variables|/Game/Widget/HUBScreen/WBP_HUBScreen.WBP_HUBScreen_C|GetPopup (Variables|/Game/Blueprint/Global/BP_TomorrowsDay_PC.BP_TomorrowsDay_PC_C|GetHUBScreen (Variables|Manager|GetTomorrows%20Day%20PC))) false)
  (Utilities|Time|SetTimerbyEvent (delegate Custom|CustomEvent) 5.0))

(event EventBeginPlay
  ;[1 1 1] Initialization Binding Event
  (CallFunction|BindInit))

(event Custom|BindAnalyseInProgress
  ;[1 1 1] Analyse Report
  (EventDispatchers|BindEventtoOnAnalyseinProgress (Variables|Manager|GetInvestigation%20Manager) (delegate Custom|AnalyseInProgress_Event)))

(event Custom|AnalyseInProgress_Event
  (params (CurrentHint :type AC%20Hint%20Information%20Object%20Reference) (HintElement :type S%20Hint%20Structure) (UVHint :type S%20Hint%20UV%20Info%20Structure) (Image :type Texture%202D%20Object%20Reference))
  ;[1 1 1] Analyse Report
  (Default|GetCurrentHint (Variables|/Game/Widget/HUBScreen/WBP_HUBScreen.WBP_HUBScreen_C|GetWBP_AnalysisReport (Variables|/Game/Blueprint/Global/BP_TomorrowsDay_PC.BP_TomorrowsDay_PC_C|GetHUBScreen (Variables|Manager|GetTomorrows%20Day%20PC))) HintElement Image))

(event Custom|BindAddSearch
  ;[1 1 1] Research Result
  (EventDispatchers|BindEventtoOnAddSearchEntry (Variables|Manager|GetData%20Manager) (delegate Custom|AddSearchEntry_Event)))

(event Custom|AddSearchEntry_Event
  (params (RowName :type Name))
  ;[1 1 1] Research Result
  (bind _returnvalue (Utilities|GetDataTableRow "/Game/DataBase/DT_Citizen.DT_Citizen" RowName)
    (:then
      (Default|AddResultButton (Variables|/Game/Widget/HUBScreen/WBP_HUBScreen.WBP_HUBScreen_C|GetWBP_DataCenter (Variables|/Game/Blueprint/Global/BP_TomorrowsDay_PC.BP_TomorrowsDay_PC_C|GetHUBScreen (Variables|Manager|GetTomorrows%20Day%20PC))) RowName (.OfficialInfo (Utilities|Struct|BreakSCitizen _returnvalue))))))

(event Custom|BindDisplayResearch
  (EventDispatchers|AssignOnDisplayResearch (Variables|Manager|GetData%20Manager) (delegate Custom|DisplayResearch_Event)))

(event Custom|DisplayResearch_Event
  (params (RowName :type Name))
  (bind _returnvalue (Utilities|GetDataTableRow (Variables|/Game/Blueprint/Global/Manager/BP_DataManager.BP_DataManager_C|GetCitizenData (Variables|Manager|GetData%20Manager)) RowName)
    (:then
      (Default|GetSearchData (Variables|/Game/Widget/HUBScreen/WBP_HUBScreen.WBP_HUBScreen_C|GetWBP_DataCenter (Variables|/Game/Blueprint/Global/BP_TomorrowsDay_PC.BP_TomorrowsDay_PC_C|GetHUBScreen (Variables|Manager|GetTomorrows%20Day%20PC))) _returnvalue)
      (CallFunction|SuspectPing RowName))))

(event Custom|SuspectPing
  (params (Suspect :type Name))
  (Variables|/Game/Widget/HUBScreen/MapDallas/WBP_Map.WBP_Map_C|SetSuspect (Variables|/Game/Widget/HUBScreen/WBP_HUBScreen.WBP_HUBScreen_C|GetWBP_Map (Variables|/Game/Blueprint/Global/BP_TomorrowsDay_PC.BP_TomorrowsDay_PC_C|GetHUBScreen (Variables|Manager|GetTomorrows%20Day%20PC))) Suspect))

(event Custom|BindClicked
  (EventDispatchers|BindEventtoOnClicked (Variables|/Game/Widget/HUBScreen/InformationsCenter/WBP_Citizen_OfficialData.WBP_Citizen_OfficialData_C|GetBut_Pin (Variables|/Game/Widget/HUBScreen/InformationsCenter/WBP_InformationsCenter.WBP_InformationsCenter_C|GetWBP_Citizen_OfficialData (Variables|/Game/Widget/HUBScreen/WBP_HUBScreen.WBP_HUBScreen_C|GetWBP_DataCenter (Variables|/Game/Blueprint/Global/BP_TomorrowsDay_PC.BP_TomorrowsDay_PC_C|GetHUBScreen (Variables|Manager|GetTomorrows%20Day%20PC))))) (delegate Custom|Click_Event)))

(event Custom|Click_Event
  (Default|DisplaySuspectPing (Variables|/Game/Widget/HUBScreen/WBP_HUBScreen.WBP_HUBScreen_C|GetWBP_Map (Variables|/Game/Blueprint/Global/BP_TomorrowsDay_PC.BP_TomorrowsDay_PC_C|GetHUBScreen (Variables|Manager|GetTomorrows%20Day%20PC))))
  (bind _asbp_cork_board (Utilities|Casting|CastToBP_CorkBoard (Utilities|Array|Get(acopy) (Variables|/Game/Blueprint/Global/Manager/BP_SceneManager.BP_SceneManager_C|GetDeskElement (Variables|Manager|GetScene%20Manager)) 2)))
  (bind _aswbp_cork_board_hud (Utilities|Casting|CastToWBP_CorkBoardHUD (UserInterface|GetWidget (Variables|/Game/Blueprint/Office/CorkBoard/BP_CorkBoard.BP_CorkBoard_C|GetWidget _asbp_cork_board))))
  (Widget|SetVisibility (Variables|/Game/Widget/CorkBoard/WBP_CorkBoardHUD.WBP_CorkBoardHUD_C|GetAmyPowels _aswbp_cork_board_hud) "Visible"))

(fn ConstructionScript)

(fn SetManagerVariable
  (bind _scene_manager (Variables|Manager|GetScene%20Manager))
  (Utilities|FlowControl|Sequence
    (:then_0
      (Variables|Manager|SetInvestigation%20Manager (Variables|/Game/Blueprint/Global/Manager/BP_SceneManager.BP_SceneManager_C|GetInvestigation%20Manager _scene_manager))
      (Variables|Manager|SetData%20Manager (Variables|/Game/Blueprint/Global/Manager/BP_SceneManager.BP_SceneManager_C|GetDataManager _scene_manager))
      (Variables|Default|SetCamera%20Manager (Variables|/Game/Blueprint/Global/Manager/BP_SceneManager.BP_SceneManager_C|GetCameraManager _scene_manager)))
    (:then_1
      (Variables|Manager|SetTomorrows%20Day%20PC (.AsBP%20Tomorrows%20Day%20PC (Utilities|Casting|CastToBP_TomorrowsDay_PC (Game|GetPlayerController 0)))))))

(fn BindAllEvent
  (CallFunction|BindAnalyseinProgress)
  (CallFunction|BindAddSearch)
  (CallFunction|BindClicked)
  (CallFunction|BindDisplayResearch)
  (CallFunction|BindArchiveSelected))