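; BP_Timer is an office actor that shows an hours-and-minutes countdown for the active investigation.
; It gets the InvestigationManager through the SceneManager singleton's initialization event and listens for investigation start, taking hours from the investigation's Duration.
; Tick drains the minute timer by delta seconds, decrementing hours and resetting it below zero, until hours run out.
; Both values feed separate WBP_Timer widget components.
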(event Custom|CountDown
  (params (deltaTime :type Float%20%28double-precision%29))
  (bind _output_get (CallFunction|TimerCondition deltaTime))
  (CallFunction|SetTimerValue (Math|Float|Truncate _output_get) (Variables|Default|GetW_MinuteTimer))
  (if (< (Variables|Default|GetCurrentTimer) 0.0)
    (bind _result (Math|Float|DecrementFloat (Variables|Default|GetHoursTimer))
      (:%20%20
        (CallFunction|SetTimerValue (Math|Float|Truncate _result) (Variables|Default|GetW_HoursTimer))
        (Variables|Default|SetCurrentTimer (Variables|Default|GetMinuteTimer))))))

(event Custom|BindInit
  ;[1 1 1] Initialization Binding Event
  (bind _output_get (Variables|Manager|SetScene%20Manager (.AsBP%20Scene%20Manager (Utilities|Casting|CastToBP_SceneManager (CallFunction|GetSingletonInstance "/Game/Blueprint/Global/Manager/BP_SceneManager.BP_SceneManager_C")))))
  (EventDispatchers|BindEventtoOnInitializationBind _output_get (delegate Custom|BindInitEvent)))

(event Custom|BindInitEvent
  ;[1 1 1] Initialization Binding Event
  (Utilities|FlowControl|Sequence
    (:then_0
      (Variables|Manager|SetInvestigation%20Manager (Variables|/Game/Blueprint/Global/Manager/BP_SceneManager.BP_SceneManager_C|GetInvestigation%20Manager (Variables|Manager|GetScene%20Manager))))
    (:then_1
      (CallFunction|BindStartInvestigation)
      (Variables|Default|SetCurrentTimer (Variables|Default|GetMinuteTimer)))))

(event Custom|BindStartInvestigation
  (EventDispatchers|BindEventtoOnStartInvestigation (Variables|Manager|GetInvestigation%20Manager) (delegate Custom|StartInvestigation_Event)))

(event Custom|StartInvestigation_Event
  (params (CurrentInvestigation :type S%20Investigation%20Order%20Structure))
  (bind _output_get (Variables|Default|SetHoursTimer (.Duration (Utilities|Struct|BreakSInvestigationOrder CurrentInvestigation))))
  (CallFunction|SetTimerValue (Math|Float|Truncate _output_get) (Variables|Default|GetW_HoursTimer))
  (Variables|Default|SetbIsInvestigationStarted true))

(event EventBeginPlay
  ;[1 1 1] Initialization Binding Event
  (CallFunction|BindInit))

(event EventTick
  (params (DeltaSeconds :type Float%20%28single-precision%29))
  ;[1 1 1] Initialization Binding Event
  (if (Variables|Default|GetbIsInvestigationStarted)
    (CallFunction|CountDown DeltaSeconds)))

(fn ConstructionScript)

(fn SetTimerValue
  (params (Timer :type Integer) (Widget :type Widget%20Component%20Object%20Reference))
  (Variables|/Game/Widget/Timer/WBP_Timer.WBP_Timer_C|SetTimer (.AsWBP%20Timer (Utilities|Casting|CastToWBP_Timer (UserInterface|GetWidget Widget))) Timer))

(fn TimerCondition
  (params (InputPin :type Float%20%28double-precision%29))
  (if (> (Variables|Default|GetHoursTimer) 0.0)
    (bind _output_get (Variables|Default|SetCurrentTimer (- (Variables|Default|GetCurrentTimer) InputPin)))
    (return _output_get)
    (else
      (Variables|Default|SetbIsInvestigationStarted false))))