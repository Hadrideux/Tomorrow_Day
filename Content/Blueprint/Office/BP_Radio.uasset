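; BP_Radio is the office radio, which plays one random propaganda broadcast when the game begins play.
; On BeginPlay it caches the BP_SceneManager singleton and reads the InvestigationData table from that manager's DataManager.
; It plays a clip from the RadioPropaganda array of the hard-coded "OwensFamilly" row as non-spatial 2D sound.
; The random index range includes the array length, so it can land one past the last clip.
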(event Custom|DisplayPropaganda
  (bind _returnvalue (Utilities|GetDataTableRow (Variables|/Game/Blueprint/Global/Manager/BP_DataManager.BP_DataManager_C|GetInvestigationData (Variables|/Game/Blueprint/Global/Manager/BP_SceneManager.BP_SceneManager_C|GetDataManager (Variables|Default|GetScene%20Manager))) "OwensFamilly")
    (:then
      (Audio|PlaySound2D (Utilities|Array|Get(acopy) (Utilities|Struct|BreakSPropaganda (.Propaganda (Utilities|Struct|BreakSDesk _returnvalue))) (Math|Random|RandomIntegerinRange 0 (Utilities|Array|Length (Utilities|Struct|BreakSPropaganda (.Propaganda (Utilities|Struct|BreakSDesk _returnvalue)))))) 1.0 1.0 0.0 0 0))))

(event EventBeginPlay
  (bind _asbp_scene_manager (Utilities|Casting|CastToBP_SceneManager (CallFunction|GetSingletonInstance "/Game/Blueprint/Global/Manager/BP_SceneManager.BP_SceneManager_C")))
  (Variables|Default|SetScene%20Manager _asbp_scene_manager)
  (CallFunction|DisplayPropaganda))

(fn ConstructionScript)