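; BP_AudioHint is a hint object whose VisualFilter component is shown only while the camera's Audio filter is selected.
; On BeginPlay it gets the BP_SceneManager singleton and waits for its binding-initiate event before subscribing to the CameraManager's filter-change event.
; Each filter change toggles the component's visibility, hiding it for None, Thermal and UV.
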(event Custom|BindInit
  (bind _output_get (CallFunction|GetSingletonInstance "/Game/Blueprint/Global/Manager/BP_SceneManager.BP_SceneManager_C"))
  (bind _asbp_scene_manager (Utilities|Casting|CastToBP_SceneManager _output_get))
  ;[1 1 1] Initialization Binding Event
  (EventDispatchers|BindEventtoOnBindingInitiate _asbp_scene_manager (delegate Custom|BindInitEvent))
  (Variables|Default|SetSceneManager _asbp_scene_manager))

(event Custom|BindInitEvent
  ;[1 1 1] Initialization Binding Event
  (CallFunction|BindCurrentFilter))

(event Custom|BindCurrentFilter
  (EventDispatchers|BindEventtoOnChangeFilter (Variables|/Game/Blueprint/Global/Manager/BP_SceneManager.BP_SceneManager_C|GetCameraManager (Variables|Default|GetSceneManager)) (delegate Custom|ChangeFitlerEvent)))

(event Custom|ChangeFitlerEvent
  (params (SelectedFilter :type EFilterType%20Enum :default "NewEnumerator0") (PostProcessIndex :type Integer))
  (switch Utilities|FlowControl|Switch|SwitchonEFilterType SelectedFilter
    (:NewEnumerator0
      (Rendering|SetVisibility (Variables|Default|GetVisualFilter) false false :!label _label))
    (:NewEnumerator1
      (Rendering|SetVisibility (Variables|Default|GetVisualFilter) true false))
    (:NewEnumerator2
      (goto _label))
    (:NewEnumerator3
      (goto _label))))

(event EventBeginPlay
  (CallFunction|BindInit))

(fn ConstructionScript)