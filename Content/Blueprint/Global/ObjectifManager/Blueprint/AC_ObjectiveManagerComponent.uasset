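; Objective manager component that holds a list of objectives and checks whether all of them are complete.
; AddObjective appends to the list and fires the OnAddedObjective dispatcher.
; From BeginPlay it binds a check to OnObjectiveComplete, which loops until it finds an incomplete objective.
; The result is only printed as debug text, with no further action on completion.
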(event Custom|AllObjectiveCompleted?
  (Variables|Default|SetChechIsBreak false)
  (bind _array_element (Utilities|Array|ForEachLoopwithBreak (Variables|Default|GetObjective) :!label _label)
    (:LoopBody
      (if (not (Variables|/Game/Blueprint/Global/ObjectifManager/Blueprint/AC_ObjectiveComponent.AC_ObjectiveComponent_C|GetIsComplete _array_element))
        (Variables|Default|SetChechIsBreak true)
        (goto _label Break)))
    (:Completed
      (if (Variables|Default|GetChechIsBreak)
        (Development|PrintString "NONE")
        (else
          (Development|PrintString "OK !"))))))

(event EventBeginPlay
  (EventDispatchers|BindEventtoOnObjectiveComplete (delegate Custom|AllObjectiveCompleted?)))

(fn AddObjective
  (params (Objective :type AC%20Objective%20Component%20Object%20Reference))
  (Utilities|Array|Add (Variables|Default|GetObjective) Objective)
  (Default|CallOnAddedObjective))