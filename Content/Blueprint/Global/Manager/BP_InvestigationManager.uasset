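; Investigation manager that runs analysis of hints, drawing on the hint data table held by the scene manager's DataManager.
; An analyse request either starts stepping through the row's hints or breaks the running analysis.
; Each hint is added to HintForAnalyse, then timed by a non-latent loop accumulating delta seconds.
; A custom breakable loop saves the stopped index, and completion or interruption fires OnAnalyseBreak.
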(event Custom|NewAnalyse
  (EventDispatchers|BindEventtoOnAnalyseRequest (delegate Custom|AnalyseInProgress)))

(event Custom|AnalyseInProgress
  (params (NewParam :type Boolean))
  (bind _hint_for_analyse (Variables|Default|GetHint%20for%20Analyse))
  (if (not NewParam)
    (Variables|Default|SetCurrentAnalyseElement _hint_for_analyse)
    (bind _returnvalue (Utilities|GetDataTableRow (Variables|/Game/Blueprint/Global/Manager/BP_DataManager.BP_DataManager_C|GetHintData (Variables|/Game/Blueprint/Global/Manager/BP_SceneManager.BP_SceneManager_C|GetDataManager (Variables|Manager|GetScene%20Manager))) (Variables|/Game/Blueprint/Hint/AC_HintInformation.AC_HintInformation_C|GetRowName _hint_for_analyse))
      (:then
        (bind (_array_element _arrayindex _arrayindexstopped) (Utilities|ForEachLoopwithBreakandBreakOutput (.Hints (Utilities|Struct|BreakSInfo_Hint _returnvalue)) (Variables|/Game/Blueprint/Hint/AC_HintInformation.AC_HintInformation_C|GetCurrentAnalyseIndex (Variables|Default|GetCurrentAnalyseElement)))
          (:LoopBody
            (Utilities|Array|Add (Variables|/Game/Blueprint/Hint/AC_HintInformation.AC_HintInformation_C|GetHint%20Information (Variables|Default|GetHint%20for%20Analyse)) _array_element)
            (CallFunction|IncrementAnalyseDuration (Variables|AnalyseDuration|GetTime%20Stage))
            (CallFunction|NextElement))
          (:Completed
            (Development|PrintString "Analyse End")
            (Default|CallOnAnalyseBreak :!label _label))
          (:Stopped
            (Variables|/Game/Blueprint/Hint/AC_HintInformation.AC_HintInformation_C|SetCurrentAnalyseIndex (Variables|Default|GetHint%20for%20Analyse) _arrayindexstopped)
            (Development|PrintString (Utilities|String|Append "Analyse break to {Index} element" (Utilities|String|ToString(Integer) _arrayindexstopped)))
            (goto _label)))))
    (else
      (CallFunction|AnalyseBreak))))

(event Custom|AnalyseBreak
  (Utilities|ForEachLoopwithBreakandBreakOutput (.Hints (Utilities|Struct|BreakSInfo_Hint (stale Custom|AnalyseInProgress _returnvalue))) (Variables|/Game/Blueprint/Hint/AC_HintInformation.AC_HintInformation_C|GetCurrentAnalyseIndex (Variables|Default|GetCurrentAnalyseElement))) ; enters at Break
)

(event Custom|NextElement
  (bind (_array_element _arrayindex _arrayindexstopped) (Utilities|ForEachLoopwithBreakandBreakOutput (.Hints (Utilities|Struct|BreakSInfo_Hint (stale Custom|AnalyseInProgress _returnvalue))) (Variables|/Game/Blueprint/Hint/AC_HintInformation.AC_HintInformation_C|GetCurrentAnalyseIndex (Variables|Default|GetCurrentAnalyseElement)))
    (:LoopBody
      (Utilities|Array|Add (Variables|/Game/Blueprint/Hint/AC_HintInformation.AC_HintInformation_C|GetHint%20Information (Variables|Default|GetHint%20for%20Analyse)) _array_element)
      (CallFunction|IncrementAnalyseDuration (Variables|AnalyseDuration|GetTime%20Stage))
      (CallFunction|NextElement))
    (:Completed
      (Development|PrintString "Analyse End")
      (Default|CallOnAnalyseBreak :!label _label))
    (:Stopped
      (Variables|/Game/Blueprint/Hint/AC_HintInformation.AC_HintInformation_C|SetCurrentAnalyseIndex (Variables|Default|GetHint%20for%20Analyse) _arrayindexstopped)
      (Development|PrintString (Utilities|String|Append "Analyse break to {Index} element" (Utilities|String|ToString(Integer) _arrayindexstopped)))
      (goto _label))))

(event EventTick
  (params (DeltaSeconds :type Float%20%28single-precision%29)))

(event EventBeginPlay
  (CallFunction|NewAnalyse)
  (Variables|Manager|SetScene%20Manager (.AsBP%20Scene%20Manager (Utilities|Casting|CastToBP_SceneManager (CallFunction|GetSingletonInstance "/Game/Blueprint/Global/Manager/BP_SceneManager.BP_SceneManager_C"))))
  (Development|PrintString (Utilities|String|ToString(Float) (Math|Float|%(Float) 3.0 6e+01))))

(fn ConstructionScript)

(fn AdditionnalInformation
  (params (NewParam :type Boolean))
  (return false))

(fn IncrementAnalyseDuration
  (params (TimeStage :type Float%20%28double-precision%29))
  (bind _output_get (LocalVariables|SetDurationStage (+ (LocalVariables|GetDurationStage) (Utilities|Time|GetWorldDeltaSeconds)) :!label _label))
  (if (> _output_get TimeStage)
    (LocalVariables|SetDurationStage 0.0)
    (return)
    (else
      (goto _label))))