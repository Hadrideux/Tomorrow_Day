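; Player controller for Tomorrow's Day that switches possession between James Steel, desk elements and the camera controller.
; A singleton scene manager supplies the desk elements, investigation and camera managers, and triggers event binding on initialization.
; Once an investigation starts, possession events blend the view, then swap pawn, widget, input mode and mapping context.
; Enhanced Input actions forward look, selection, hint, cork board and leave commands through event calls.
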(event Custom|BindInit
  (bind _returnvalue (PlayerController|LocalPlayerSubsystems|GetEnhancedInputLocalPlayerSubsystem))
  ;[1 1 1] Initialization Binding Event
  (bind _output_get (Variables|Manager|SetScene%20Manager (.AsBP%20Scene%20Manager (Utilities|Casting|CastToBP_SceneManager (CallFunction|GetSingletonInstance "/Game/Blueprint/Global/Manager/BP_SceneManager.BP_SceneManager_C")))))
  (EventDispatchers|BindEventtoOnInitializationBind _output_get (delegate Custom|BindInitEvent))
  (Input|AddMappingContext _returnvalue "/Game/Blueprint/Character/Input/IMC_CharacterDefault.IMC_CharacterDefault" 0 "(bIgnoreAllPressedKeysUntilRelease=True,bForceImmediately=False,bNotifyUserSettings=False)")
  (Input|AddMappingContext _returnvalue "/Game/Blueprint/Character/Input/IMC_Debug.IMC_Debug" 1 "(bIgnoreAllPressedKeysUntilRelease=True,bForceImmediately=False,bNotifyUserSettings=False)")
  (CallFunction|InitializeCreatingWidget))

(event Custom|BindInitEvent
  ;[1 1 1] Initialization Binding Event
  (Utilities|FlowControl|Sequence
    (:then_0
      (Init|SetManagerVariable)
      (Input|SetInputModeGameOnly self false))
    (:then_1
      (Init|BindAllEvent))))

(event Input|EnhancedActionEvents|EnhancedInputActionIA_LookAt
  (params (ActionValue :type Vector%202D%20Structure) (ElapsedSeconds :type Float%20%28double-precision%29) (TriggeredSeconds :type Float%20%28double-precision%29) (InputAction :type Input%20Action%20Object%20Reference :default "/Game/Blueprint/Character/Input/Action/Game/IA_LookAt.IA_LookAt"))
  (bind _crosshair (Variables|Default|GetCrosshair))
  (if (== (Variables|Default|GetCurrentPossess) (Variables|Default|GetJamesSteel))
    (Default|CallOnLookAround ActionValue)
    (if (not (UserInterface|Viewport|IsinViewport _crosshair))
      (UserInterface|Viewport|AddtoViewport _crosshair 0))
    (else
      (Widget|RemovefromParent (Variables|Default|GetCrosshair)))))

(event Input|EnhancedActionEvents|EnhancedInputActionIA_Focus
  (params (ActionValue :type Vector%202D%20Structure) (ElapsedSeconds :type Float%20%28double-precision%29) (TriggeredSeconds :type Float%20%28double-precision%29) (InputAction :type Input%20Action%20Object%20Reference :default "/Game/Blueprint/Character/Input/Action/Game/IA_Focus.IA_Focus"))
  (Default|CallOnFocusHint))

(event Input|EnhancedActionEvents|EnhancedInputActionIA_AnalysesFocus
  (params (ActionValue :type Boolean) (ElapsedSeconds :type Float%20%28double-precision%29) (TriggeredSeconds :type Float%20%28double-precision%29) (InputAction :type Input%20Action%20Object%20Reference :default "/Game/Blueprint/Character/Input/Action/Game/IA_AnalysesFocus.IA_AnalysesFocus"))
  (:Started
    (Default|CallOnAnalyseHint)))

(event Input|EnhancedActionEvents|EnhancedInputActionIA_ShowHintSheet
  (params (ActionValue :type Boolean) (ElapsedSeconds :type Float%20%28double-precision%29) (TriggeredSeconds :type Float%20%28double-precision%29) (InputAction :type Input%20Action%20Object%20Reference :default "/Game/Blueprint/Character/Input/Action/Debug/IA_ShowHintSheet.IA_ShowHintSheet"))
  (:Started
    (Default|CallOnPrintAnalyse (Variables|Default|GetInvestigation%20Manager))))

(event Input|EnhancedActionEvents|EnhancedInputActionIA_SelectionCharacter
  (params (ActionValue :type Boolean) (ElapsedSeconds :type Float%20%28double-precision%29) (TriggeredSeconds :type Float%20%28double-precision%29) (InputAction :type Input%20Action%20Object%20Reference :default "/Game/Blueprint/Character/Input/Action/Game/IA_SelectionCharacter.IA_SelectionCharacter"))
  (:Started
    (if (== (Variables|Default|GetCurrentPossess) (Variables|Default|GetJamesSteel))
      (Default|CallOnSelection))))

(event Input|EnhancedActionEvents|EnhancedInputActionIA_CorkBoard
  (params (ActionValue :type Boolean) (ElapsedSeconds :type Float%20%28double-precision%29) (TriggeredSeconds :type Float%20%28double-precision%29) (InputAction :type Input%20Action%20Object%20Reference :default "/Game/Blueprint/Character/Input/Action/Debug/IA_CorkBoard.IA_CorkBoard"))
  (:Triggered
    (bind _asbp_cork_board (Utilities|Casting|CastToBP_CorkBoard (CallFunction|GetDeskElementArray 2)))
    (Default|OnPrintAnalyseEvent _asbp_cork_board)))

(event EventBeginPlay
  ;[1 1 1] Initialization Binding Event
  (CallFunction|BindInit))

(event Custom|LeavePossessCamera
  (params (Dimension%201 :type Integer))
  (Pawn|Possess (CallFunction|GetDeskElementArray Dimension%201))
  (CallFunction|NewPossess (CallFunction|GetDeskElementArray)))

(event Custom|NewPossess
  (params (Pawn :type Pawn%20Object%20Reference))
  (bind _hubscreen (Variables|Widget|GetHUBScreen))
  (if (Variables|/Game/Blueprint/Global/Manager/BP_InvestigationManager.BP_InvestigationManager_C|GetbIsInvestigationStarted (Variables|Default|GetInvestigation%20Manager))
    (bind _output_get (Variables|Default|SetCurrentPossess Pawn))
    (CallFunction|PossessNewPawn _output_get)
    (Utilities|FlowControl|Delay 0.55)
    (if (!= (Variables|Default|GetCurrentPossess) (Variables|Default|GetJamesSteel))
      (if (CallFunction|ComparePossess)
        (UserInterface|Viewport|AddtoViewport _hubscreen 0)
        (Variables|Default|SetCurrentActiveWidget _hubscreen)
        (elif (and (CallFunction|ComparePossess 1) (Variables|/Game/Blueprint/Global/Manager/BP_CameraManager.BP_CameraManager_C|GetbIsArchiveIsSelected (Variables|Manager|GetCamera%20Manager)))
          (CallFunction|PossessCameraController))))))

(event Custom|PossessNewPawn
  (params (PawnPossess :type Pawn%20Object%20Reference))
  ;[1 1 1] Possess New Pawn
  (CallFunction|SetPossessTransistion PawnPossess)
  (Utilities|FlowControl|Delay 0.55)
  (Pawn|Possess PawnPossess)
  (if (!= PawnPossess (Variables|Default|GetJamesSteel))
    (CallFunction|SetPlayerConfig true "/Game/Blueprint/Character/Input/IMC_Camera.IMC_Camera" "/Game/Blueprint/Character/Input/IMC_CharacterDefault.IMC_CharacterDefault")
    (Input|SetInputModeGameandUI self (Variables|Default|GetCurrentActiveWidget) "DoNotLock" true false)
    (else
      (CallFunction|SetPlayerConfig false "/Game/Blueprint/Character/Input/IMC_Camera.IMC_Camera" "/Game/Blueprint/Character/Input/IMC_CharacterDefault.IMC_CharacterDefault")
      (Input|SetInputModeGameOnly self false))))

(event Custom|BindLeaveScreen
  ;[1 1 1] Return to James Steel
  (EventDispatchers|BindEventtoOnLeaveScreen (delegate Custom|LeaveScreen_Event)))

(event Custom|SetPossessTransistion
  (params (PawnPossessed :type Pawn%20Object%20Reference))
  ;[1 1 1] Possess New Pawn
  (Game|Player|SetViewTargetwithBlend PawnPossessed 0.5 "VTBlend_EaseOut" 1.25 false)
  (CallFunction|RemoveCurrentWidget))

(event Custom|PossessCharacter
  (params (DeskElementIndex :type Integer))
  (Pawn|Possess (CallFunction|GetDeskElementArray DeskElementIndex))
  (CallFunction|LeaveScreenEvent))

(event Custom|BindNewPossess
  (EventDispatchers|BindEventtoOnNewPossessPawn (delegate Custom|NewPossess)))

(event Custom|LeaveScreen_Event
  (bind _jamessteel (Variables|Default|GetJamesSteel))
  ;[1 1 1] Return to James Steel
  (CallFunction|PossessNewPawn _jamessteel)
  (Variables|Default|SetCurrentPossess _jamessteel))

(event Input|EnhancedActionEvents|EnhancedInputActionIA_LeavePawn
  (params (ActionValue :type Boolean) (ElapsedSeconds :type Float%20%28double-precision%29) (TriggeredSeconds :type Float%20%28double-precision%29) (InputAction :type Input%20Action%20Object%20Reference :default "/Game/Blueprint/Character/Input/Action/Game/IA_LeavePawn.IA_LeavePawn"))
  (:Started
    (Default|CallOnLeaveScreen)))

(fn ConstructionScript)

(fn InitializeCreatingWidget
  (Utilities|FlowControl|Sequence
    (:then_0
      ;[1 1 1] Main Interface
      (bind _returnvalue (UserInterface|CreateWidget "/Game/Widget/HUBScreen/WBP_HUBScreen.WBP_HUBScreen_C"))
      (Variables|Widget|SetHUBScreen _returnvalue)
      (bind _returnvalue_2 (UserInterface|CreateWidget "/Game/Widget/RegisScreen/WBP_RegisInterface.WBP_RegisInterface_C"))
      (Variables|Widget|SetRegisScreen _returnvalue_2)
      (bind _returnvalue_3 (UserInterface|CreateWidget "/Game/Widget/CorkBoard/WBP_CorkBoardHUD.WBP_CorkBoardHUD_C"))
      (Variables|Widget|SetCorkBoard _returnvalue_3))
    (:then_1
      ;[1 1 1] Camera Interface
      (bind _returnvalue_4 (UserInterface|CreateWidget "/Game/Widget/Camera/WBP_CameraInterface.WBP_CameraInterface_C"))
      (Variables|Widget|SetCameraInterface _returnvalue_4))
    (:then_2
      (bind _returnvalue_5 (UserInterface|CreateWidget "/Game/Widget/WBP_Crosshair.WBP_Crosshair_C"))
      (Variables|Default|SetCrosshair _returnvalue_5))))

(fn SetPlayerConfig
  (params (Show%20Mouse%20Cursor :type Boolean) (RemovePreviousMapping :type Input%20Mapping%20Context%20Object%20Reference) (AddNewMapping :type Input%20Mapping%20Context%20Object%20Reference))
  (bind _returnvalue (PlayerController|LocalPlayerSubsystems|GetEnhancedInputLocalPlayerSubsystem))
  (Variables|Default|SetbShowMouseCursor Show%20Mouse%20Cursor)
  (Input|RemoveMappingContext _returnvalue RemovePreviousMapping "(bIgnoreAllPressedKeysUntilRelease=True,bForceImmediately=False,bNotifyUserSettings=False)")
  (Input|AddMappingContext _returnvalue AddNewMapping 0 "(bIgnoreAllPressedKeysUntilRelease=True,bForceImmediately=False,bNotifyUserSettings=False)"))

(fn SetManagerVariable
  (bind _scene_manager (Variables|Manager|GetScene%20Manager))
  (Utilities|FlowControl|Sequence
    (:then_0
      (Variables|Manager|SetCamera%20Manager (Variables|/Game/Blueprint/Global/Manager/BP_SceneManager.BP_SceneManager_C|GetCameraManager _scene_manager))
      (Variables|Default|SetInvestigation%20Manager (Variables|/Game/Blueprint/Global/Manager/BP_SceneManager.BP_SceneManager_C|GetInvestigation%20Manager _scene_manager)))))

(fn BindAllEvent
  (CallFunction|BindNEwPossess)
  (CallFunction|BindLeaveScreen))

(fn GetDeskElementArray
  (params (DeskElementIndex :type Integer))
  (return (Utilities|Array|Get(acopy) (Variables|/Game/Blueprint/Global/Manager/BP_SceneManager.BP_SceneManager_C|GetDeskElement (.AsBP%20Scene%20Manager (Utilities|Casting|CastToBP_SceneManager (CallFunction|GetSingletonInstance "/Game/Blueprint/Global/Manager/BP_SceneManager.BP_SceneManager_C")))) DeskElementIndex)))

(fn PossessCameraController
  (bind _camerainterface (Variables|Widget|GetCameraInterface))
  (Pawn|Possess (Variables|/Game/Blueprint/Global/Manager/BP_CameraManager.BP_CameraManager_C|GetCameraController (Variables|/Game/Blueprint/Global/Manager/BP_SceneManager.BP_SceneManager_C|GetCameraManager (.AsBP%20Scene%20Manager (Utilities|Casting|CastToBP_SceneManager (CallFunction|GetSingletonInstance "/Game/Blueprint/Global/Manager/BP_SceneManager.BP_SceneManager_C"))))))
  (UserInterface|Viewport|AddtoViewport _camerainterface 0)
  (Variables|Default|SetCurrentActiveWidget _camerainterface)
  (CallFunction|SetPlayerConfig true "/Game/Blueprint/Character/Input/IMC_CharacterDefault.IMC_CharacterDefault" "/Game/Blueprint/Character/Input/IMC_Camera.IMC_Camera")
  (Input|SetInputModeGameandUI self (Variables|Default|GetCurrentActiveWidget) "DoNotLock" false true))

(fn RemoveCurrentWidget
  (bind _currentactivewidget (Variables|Default|GetCurrentActiveWidget))
  (Utilities|IsValid _currentactivewidget
    (:Is%20Valid
      (Widget|RemovefromParent _currentactivewidget))))

(fn ComparePossess
  (params (DeskElementIndex :type Integer))
  (return (== (Variables|Default|GetCurrentPossess) (CallFunction|GetDeskElementArray DeskElementIndex))))