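; BP_Interactable is an interactable world object that shows a UI prompt when something is near it.
; On BeginPlay it looks up its data table row through DataRowHandle and applies that row's mesh to the Cube component.
; Box overlaps toggle the Widget's visibility without filtering the overlapping actor.
; While visible, Tick turns the widget toward the player character; no interaction action is implemented here.
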(event OnComponentBeginOverlap(Box)
  (params (OverlappedComponent :type Primitive%20Component%20Object%20Reference) (OtherActor :type Actor%20Object%20Reference) (OtherComp :type Primitive%20Component%20Object%20Reference) (OtherBodyIndex :type Integer) (bFromSweep :type Boolean) (SweepResult :type Hit%20Result%20Structure%20%28by%20ref%29))
  ;[1 1 1] Display UI Interact
  (bind _output_get (Variables|UI|SetIsVisible true))
  (Rendering|SetVisibility (Variables|Default|GetWidget) _output_get false))

(event OnComponentEndOverlap(Box)
  (params (OverlappedComponent :type Primitive%20Component%20Object%20Reference) (OtherActor :type Actor%20Object%20Reference) (OtherComp :type Primitive%20Component%20Object%20Reference) (OtherBodyIndex :type Integer))
  ;[1 1 1] Display UI Interact
  (bind _output_get (Variables|UI|SetIsVisible false))
  (Rendering|SetVisibility (Variables|Default|GetWidget) _output_get false))

(event Custom|RotationUI
  ;[1 1 1] Target Rotation UI To Character
  (if (Variables|UI|GetIsVisible)
    (Transformation|SetWorldRotation (Variables|Default|GetWidget) (Math|Rotator|FindLookatRotation (Transformation|GetActorLocation) (Transformation|GetActorLocation (Game|GetPlayerCharacter 0))) false false)))

(event EventBeginPlay
  (bind _out_row (CallFunction|GetDataRessource self))
  (Components|StaticMesh|SetStaticMesh (Variables|Default|GetCube) (.Mesh (Utilities|Struct|BreakS_Ressource _out_row))))

(event EventTick
  (params (DeltaSeconds :type Float%20%28single-precision%29))
  (if (Variables|UI|GetIsVisible)
    (CallFunction|RotationUI)))

(fn ConstructionScript)

(fn GetDataRessource
  (bind _data_rowhandle (Variables|Data|GetData%20RowHandle))
  (bind (_datatable _rowname) (Utilities|Struct|BreakDataTableRowHandle _data_rowhandle))
  (bind _returnvalue (Utilities|GetDataTableRow _datatable _rowname)
    (:then
      (return _rowname _returnvalue))))