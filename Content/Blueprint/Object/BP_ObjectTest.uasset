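; BP_ObjectTest is a test world object that shows an interact widget when something overlaps its box.
; Box overlap begin and end set IsVisible and toggle the widget's visibility, with no check on the overlapping actor.
; While visible, Tick rotates the widget toward the player character using a look-at rotation from the actor's location.
; BeginPlay assigns a random integer EnergyIntake, which this file does not otherwise use.
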(event OnComponentBeginOverlap(Box)
  (params (OverlappedComponent :type Primitive%20Component%20Object%20Reference) (OtherActor :type Actor%20Object%20Reference) (OtherComp :type Primitive%20Component%20Object%20Reference) (OtherBodyIndex :type Integer) (bFromSweep :type Boolean) (SweepResult :type Hit%20Result%20Structure%20%28by%20ref%29))
  ;[1 1 1] Display UI Interact
  (bind _output_get (Variables|UI|SetIsVisible true))
  (Rendering|SetVisibility (Variables|Default|GetWidget) _output_get false))

(event OnComponentEndOverlap(Box)
  (params (OverlappedComponent :type Primitive%20Component%20Object%20Reference) (OtherActor :type Actor%20Object%20Reference) (OtherComp :type Primitive%20Component%20Object%20Reference) (OtherBodyIndex :type Integer))
  ;[1 1 1] Display UI Interact
  (bind _output_get (Variables|UI|SetIsVisible false))
  (Rendering|SetVisibility (Variables|Default|GetWidget) _output_get false))

(event Custom|RotationUI
  ;[1 1 1] Target Rotation UI To Character
  (if (Variables|UI|GetIsVisible)
    (Transformation|SetWorldRotation (Variables|Default|GetWidget) (Math|Rotator|FindLookatRotation (Transformation|GetActorLocation) (Transformation|GetActorLocation (Game|GetPlayerCharacter 0))) false false)))

(event EventBeginPlay
  (Variables|Energy|SetEnergyIntake (Math|Random|RandomIntegerinRange 5 20)))

(event EventTick
  (params (DeltaSeconds :type Float%20%28single-precision%29))
  (if (Variables|UI|GetIsVisible)
    (CallFunction|RotationUI)))

(fn ConstructionScript)