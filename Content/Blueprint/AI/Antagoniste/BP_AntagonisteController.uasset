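; Antagonist AI pawn with player sighting through PawnSensing and a ForceKillAntagoniste input for removing it.
; Pressing that input asks the Manager to delay spawning, and releasing it destroys the actor.
; BeginPlay and sighting any pawn, which sets IsSeePlayer, both call MoveTo, but that event is empty.
; The chase-player or random-wander AIMoveTo logic is disconnected and never runs.
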(event OnSeePawn(PawnSensing)
  (params (Pawn :type Pawn%20Object%20Reference))
  ;[1 1 1] IA Set Destination Move To
  (Variables|Default|SetIsSeePlayer true)
  (CallFunction|Moveto))

(event Custom|MoveTo
  ;[1 1 1] IA Set Destination Move To
)

(event EventBeginPlay
  (CallFunction|Moveto))

(event Input|ActionEvents|InputActionForceKillAntagoniste
  (params (Key :type Key%20Structure :default "None"))
  (:Pressed
    (Default|DelaySpawn (Variables|Default|GetManager)))
  (:Released
    (Actor|DestroyActor)))

(fn ConstructionScript)