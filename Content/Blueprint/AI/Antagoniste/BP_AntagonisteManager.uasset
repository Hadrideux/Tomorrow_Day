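; BP_AntagonisteManager spawns the Antagoniste AI into the level at a random place and time.
; On BeginPlay, DelaySpawn checks the IsSpawn flag and, if nothing has spawned, waits a random delay of up to ten seconds.
; SpawnPointRandom then spawns one Antagoniste at the location of a randomly picked entry in the SpawnPoint array and sets IsSpawn.
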(event Custom|SpawnPointRandom
  ;[1 1 1] Random Spawn at SpawnPoint
  (Game|SpawnActorfromClass (Variables|Spawn|GetAntagoniste) (Math|Transform|MakeTransform (Transformation|GetActorLocation (.OutItem (Utilities|Array|Random (Variables|Spawn|GetSpawnPoint)))) "0, 0, 0" "1.000000,1.000000,1.000000") "Undefined" 0 0)
  (Variables|Spawn|SetIsSpawn true))

(event Custom|DelaySpawn
  ;[1 1 1] Random Time Spawn
  (if (not (Variables|Spawn|GetIsSpawn))
    (Utilities|FlowControl|Delay (Math|Random|RandomFloatinRange 0.0 1e+01))
    (CallFunction|SpawnPointRandom)))

(event EventBeginPlay
  (CallFunction|DelaySpawn))

(fn ConstructionScript)