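; Player controller for the investigation desk prototype, switching the player between a character and a camera view.
; On BeginPlay it shows the cursor, adds the desk input context and creates the OS, camera and desk-camera widgets, the last not displayed here.
; IA_ChangeScreen flip-flops possession between singleton-fetched BP_Characrer and BP_Camera, swapping OS and camera interfaces.
; IA_NewSuspect reveals the second suspect on the OS map.
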(event Input|EnhancedActionEvents|EnhancedInputActionIA_NewSuspect
  (params (ActionValue :type Boolean) (ElapsedSeconds :type Float%20%28double-precision%29) (TriggeredSeconds :type Float%20%28double-precision%29) (InputAction :type Input%20Action%20Object%20Reference :default "/Game/ProtoMeca_2/Bureau_Enquête/Bureau/CharacterTest/Input/Action/IA_NewSuspect.IA_NewSuspect"))
  (:Started
    (Widget|SetVisibility (Variables|/Game/UI_UX/Widget/WBP_Map.WBP_Map_C|GetSuspect2 (Variables|/Game/ProtoMeca_2/Bureau_Enquête/Widget/WBP_OSInterface.WBP_OSInterface_C|GetWBP_Map (Variables|Default|GetHUBScreen))) "Visible")))

(event Input|EnhancedActionEvents|EnhancedInputActionIA_ChangeScreen
  (params (ActionValue :type Boolean) (ElapsedSeconds :type Float%20%28double-precision%29) (TriggeredSeconds :type Float%20%28double-precision%29) (InputAction :type Input%20Action%20Object%20Reference :default "/Game/ProtoMeca_2/Bureau_Enquête/Bureau/CharacterTest/Input/Action/IA_ChangeScreen.IA_ChangeScreen"))
  (bind _self self)
  (bind _camerainterface (Variables|Default|GetCameraInterface))
  (bind _hubscreen (Variables|Default|GetHUBScreen))
  (:Started
    (Utilities|FlowControl|FlipFlop
      (:A
        (Pawn|Possess _self (.AsBP%20Characrer (Utilities|Casting|CastToBP_Characrer (CallFunction|GetSingletonInstance "/Game/ProtoMeca_2/Bureau_Enquête/Bureau/CharacterTest/BP_Characrer.BP_Characrer_C"))))
        (Widget|RemovefromParent _camerainterface)
        (UserInterface|Viewport|AddtoViewport _hubscreen 0))
      (:B
        (Pawn|Possess _self (.AsBP%20Camera (Utilities|Casting|CastToBP_Camera (CallFunction|GetSingletonInstance "/Game/ProtoMeca_2/CameraV2/Character/BP_Camera.BP_Camera_C"))))
        (UserInterface|Viewport|AddtoViewport _camerainterface 0)
        (Widget|RemovefromParent _hubscreen)))))

(event EventBeginPlay
  (Variables|Default|SetbShowMouseCursor true)
  (Input|AddMappingContext (PlayerController|LocalPlayerSubsystems|GetEnhancedInputLocalPlayerSubsystem) "/Game/ProtoMeca_2/Bureau_Enquête/Bureau/CharacterTest/Input/IMC_CharacterDeskDefault.IMC_CharacterDeskDefault" 0 "(bIgnoreAllPressedKeysUntilRelease=True,bForceImmediately=False,bNotifyUserSettings=False)")
  (Utilities|FlowControl|Sequence
    (:then_0
      (bind _returnvalue (UserInterface|CreateWidget "/Game/ProtoMeca_2/Bureau_Enquête/Widget/WBP_OSInterface.WBP_OSInterface_C"))
      (Variables|Default|SetHUBScreen _returnvalue)
      (bind _returnvalue_2 (UserInterface|CreateWidget "/Game/ProtoMeca_2/CameraV2/Widget/WBP_CameraDeskTest_Interface.WBP_CameraDeskTest_Interface_C"))
      (Variables|Default|SetRegisScreen _returnvalue_2))
    (:then_1
      (bind _returnvalue_3 (UserInterface|CreateWidget "/Game/ProtoMeca_2/CameraV2/Widget/WBP_CameraTest_Interface.WBP_CameraTest_Interface_C"))
      (Variables|Default|SetCameraInterface _returnvalue_3))))

(fn ConstructionScript)