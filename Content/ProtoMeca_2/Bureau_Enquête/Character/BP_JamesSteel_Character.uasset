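; Player character James Steel, with first-person style move and look input plus two toggled modes, Focus and Work.
; Focus blocks movement, aims the camera at a BP_CharacterLookAt actor, shows the cursor and opens the controller's OS interface widget.
; Work blocks movement and look; each tick it moves that actor to the mouse's line-trace hit and turns the camera toward it.
; The camera rotation clamp is currently unused.
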(event Input|EnhancedActionEvents|EnhancedInputActionIA_LookAt
  (params (ActionValue :type Vector%202D%20Structure) (ElapsedSeconds :type Float%20%28double-precision%29) (TriggeredSeconds :type Float%20%28double-precision%29) (InputAction :type Input%20Action%20Object%20Reference :default "/Game/ProtoMeca_2/Bureau_Enquête/Character/Input/Action/IA_LookAt.IA_LookAt"))
  ;[1 1 1] OLD
)

(event Input|EnhancedActionEvents|EnhancedInputActionIA_FocusMode
  (params (ActionValue :type Boolean) (ElapsedSeconds :type Float%20%28double-precision%29) (TriggeredSeconds :type Float%20%28double-precision%29) (InputAction :type Input%20Action%20Object%20Reference :default "/Game/ProtoMeca_2/Bureau_Enquête/Character/Input/Action/IA_FocusMode.IA_FocusMode"))
  (bind _returnvalue (Game|GetPlayerController 0))
  (:Started
    (Utilities|FlowControl|FlipFlop
      (:A
        (Focus|Focuson)
        (Focus|FocusMode)
        (Variables|/Script/Engine.PlayerController|SetbShowMouseCursor _returnvalue true))
      (:B
        (Focus|FocusOff)
        (Variables|/Script/Engine.PlayerController|SetbShowMouseCursor _returnvalue false)))))

(event Input|EnhancedActionEvents|EnhancedInputActionIA_Movement
  (params (ActionValue :type Vector%202D%20Structure) (ElapsedSeconds :type Float%20%28double-precision%29) (TriggeredSeconds :type Float%20%28double-precision%29) (InputAction :type Input%20Action%20Object%20Reference :default "/Game/ProtoMeca_2/Bureau_Enquête/Character/Input/Action/IA_Movement.IA_Movement"))
  (if (and (not (Work|IsonWork)) (not (Focus|IsonFocus)))
    (Pawn|Input|AddMovementInput (Transformation|GetActorForwardVector) (.x ActionValue) false)
    (Pawn|Input|AddMovementInput (Transformation|GetActorRightVector) (.y ActionValue) false)))

(event Input|EnhancedActionEvents|EnhancedInputActionIA_WorkMode
  (params (ActionValue :type Boolean) (ElapsedSeconds :type Float%20%28double-precision%29) (TriggeredSeconds :type Float%20%28double-precision%29) (InputAction :type Input%20Action%20Object%20Reference :default "/Game/ProtoMeca_2/Bureau_Enquête/Character/Input/Action/IA_WorkMode.IA_WorkMode"))
  (:Started
    (Utilities|FlowControl|FlipFlop
      (:A
        (Work|StartWork)
        (Work|OnWork))
      (:B
        (Work|EndWork)))))

(event Input|EnhancedActionEvents|EnhancedInputActionIA_LookAt
  (params (ActionValue :type Vector%202D%20Structure) (ElapsedSeconds :type Float%20%28double-precision%29) (TriggeredSeconds :type Float%20%28double-precision%29) (InputAction :type Input%20Action%20Object%20Reference :default "/Game/ProtoMeca_2/Bureau_Enquête/Character/Input/Action/IA_LookAt.IA_LookAt"))
  (if (not (Work|IsonWork))
    (Pawn|Input|AddControllerYawInput (.x ActionValue))
    (Pawn|Input|AddControllerPitchInput (.y ActionValue))))

(event EventTick
  (params (DeltaSeconds :type Float%20%28single-precision%29))
  (if (Work|IsonWork)
    (bind _location (CallFunction|ConvertMouseLocationtoWorldSpace))
    (Transformation|SetActorLocation (Variables|Default|GetLookAt) _location false false)
    (Focus|CameraFocus)))

(event EventBeginPlay
  (bind _returnvalue (Actor|GetActorOfClass "/Game/ProtoMeca_2/Bureau_Enquête/Character/BP_CharacterLookAt.BP_CharacterLookAt_C"))
  (Variables|Default|SetLookAt _returnvalue))

(fn ConstructionScript)

(fn ClampRotationCamera
  (bind _returnvalue (Game|GetPlayerCameraManager 0))
  (if (Work|IsonWork)
    (Utilities|FlowControl|Sequence
      (:then_0
        (Variables|/Script/Engine.PlayerCameraManager|SetViewPitchMax _returnvalue 45.0)
        (Variables|/Script/Engine.PlayerCameraManager|SetViewPitchMin _returnvalue -45.0))
      (:then_1
        (Variables|/Script/Engine.PlayerCameraManager|SetViewYawMax _returnvalue 65.0)
        (Variables|/Script/Engine.PlayerCameraManager|SetViewYawMin _returnvalue -65.0)))))

(fn Focuson
  (Variables|Default|SetIsFocus true)
  (OSInterface|OpenInterface))

(fn FocusOff
  (Variables|Default|SetIsFocus false)
  (OSInterface|CloseInterface))

(fn IsonFocus
  (return (Variables|Default|GetIsFocus)))

(fn FocusMode
  (Focus|CameraFocus))

(fn CameraFocus
  (Transformation|SetWorldRotation (Variables|Default|GetCamera) (Math|Rotator|FindLookatRotation (Transformation|GetActorLocation) (Transformation|GetActorLocation (Variables|Default|GetLookAt))) false false))

(fn OpenInterface
  (bind _asbp_james_steel_player_controller (Utilities|Casting|CastToBP_JamesSteel_PlayerController (Game|GetPlayerController 0)))
  (UserInterface|Viewport|AddtoViewport (Variables|/Game/ProtoMeca_2/Bureau_Enquête/Character/BP_JamesSteel_PlayerController.BP_JamesSteel_PlayerController_C|GetOSInterfaceWidget _asbp_james_steel_player_controller) 0))

(fn CloseInterface
  (bind _asbp_james_steel_player_controller (Utilities|Casting|CastToBP_JamesSteel_PlayerController (Game|GetPlayerController 0)))
  (Widget|RemovefromParent (Variables|/Game/ProtoMeca_2/Bureau_Enquête/Character/BP_JamesSteel_PlayerController.BP_JamesSteel_PlayerController_C|GetOSInterfaceWidget _asbp_james_steel_player_controller)))

(fn StartWork
  (Variables|Default|SetIsWorking true))

(fn EndWork
  (Variables|Default|SetIsWorking false))

(fn IsonWork
  (return (Variables|Default|GetIsWorking)))

(fn OnWork
  (Transformation|SetActorLocation (Transformation|GetActorLocation) false true))

(fn ConvertMouseLocationtoWorldSpace
  (bind _returnvalue (Game|GetPlayerController 0))
  (bind (_worldlocation _worlddirection) (Game|Player|ConvertMouseLocationToWorldSpace _returnvalue))
  (bind _outhit (Collision|LineTraceByChannel _worldlocation (+ _worldlocation (* _worlddirection 1000)) "TraceTypeQuery1" true 0 "ForDuration"))
  (return (.Location (Collision|BreakHitResult _outhit))))

(fn GetCameraLocation)