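; Camera test pawn for inspecting hints with the mouse and switching between audio, thermal and UV view filters.
; The hint selection input line-traces under the cursor and shows or hides the camera UI's AnalyseHint from the hit BP_HintTest's TypeHint.
; The same input, not BeginPlay, binds the UI's filter events, which swap the camera's post-process settings from an indexed array, including a no-filter entry.
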(event Custom|AudioFiltre
  (Utilities|SetPostProcess))

(event Custom|ThermiqueFiltre
  (Utilities|SetPostProcess 1))

(event Custom|UVFiltre
  (Utilities|SetPostProcess 2))

(event Custom|NoFiltre
  (Utilities|SetPostProcess 3))

(event Input|EnhancedActionEvents|EnhancedInputActionIA_HintSelection
  (params (ActionValue :type Boolean) (ElapsedSeconds :type Float%20%28double-precision%29) (TriggeredSeconds :type Float%20%28double-precision%29) (InputAction :type Input%20Action%20Object%20Reference :default "/Game/ProtoMeca_2/CameraV2/Character/Input/Action/IA_HintSelection.IA_HintSelection"))
  (:Started
    (Utilities|FlowControl|Sequence
      (:then_0
        (bind _hitactor (CallFunction|MousePositiontoWorldLocation))
        (bind _asbp_hint_test (Utilities|Casting|CastToBP_HintTest _hitactor))
        (if (Variables|/Game/ProtoMeca_2/CameraV2/Hint/BP_HintTest.BP_HintTest_C|GetTypeHint _asbp_hint_test)
          (CallFunction|DisplayAnalysOption "Visible")
          (else
            (CallFunction|DisplayAnalysOption "Hidden"))))
      (:then_1
        (bind _camerainterface (Utilities|GetCameraPlayerController))
        (EventDispatchers|BindEventtoOnAudioFiltre _camerainterface (delegate Custom|AudioFiltre))
        (EventDispatchers|BindEventtoOnThermiqueFiltre _camerainterface (delegate Custom|ThermiqueFiltre))
        (EventDispatchers|BindEventtoOnUVFiltre _camerainterface (delegate Custom|UVFiltre))
        (EventDispatchers|BindEventtoNoFiltre _camerainterface (delegate Custom|NoFiltre))))))

(event EventBeginPlay)

(fn ConstructionScript)

(fn MousePositiontoWorldLocation
  (bind _returnvalue (Game|GetPlayerController 0))
  (bind (_worldlocation _worlddirection) (Game|Player|ConvertMouseLocationToWorldSpace _returnvalue))
  (bind _outhit (Collision|LineTraceByChannel _worldlocation (+ _worldlocation (* _worlddirection 1e+03)) "TraceTypeQuery1" true 0 "ForDuration"))
  (return (.HitActor (Collision|BreakHitResult _outhit))))

(fn DisplayAnalysOption
  (params (InSetVisibility :type ESlateVisibility%20Enum :default "Visible"))
  (bind _camerainterface (Utilities|GetCameraPlayerController))
  (Widget|SetVisibility (Variables|/Game/ProtoMeca_2/CameraV2/Widget/WBP_CameraTest_Interface.WBP_CameraTest_Interface_C|GetAnalyseHint _camerainterface) InSetVisibility))