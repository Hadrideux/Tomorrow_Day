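; Surveillance-style camera Blueprint that moves between preset location actors and lets the player select hints.
; The selection input line-traces under the mouse and toggles the camera UI's analyse option from the hit hint's TypeHint.
; It binds to UI filter events, sending post-process settings and its scene capture to ACAudioFilter for audio and no-filter views.
; Thermal, UV and timeline handlers are empty; a possession change adds the camera UI to the viewport.
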(event Custom|AudioFiltre
  (Default|SetView (Variables|Default|GetAC_AudioFilter) (Utilities|Array|Get(acopy) (Variables|Default|Getpostprocess)) (Variables|Default|GetSceneCaptureComponent2D) "NewEnumerator1"))

(event Custom|ThermiqueFiltre)

(event Custom|UVFiltre)

(event Custom|NoFiltre
  (Default|SetView (Variables|Default|GetAC_AudioFilter) (Utilities|Array|Get(acopy) (Variables|Default|Getpostprocess) 3) (Variables|Default|GetSceneCaptureComponent2D) "NewEnumerator0"))

(event Custom|ChangeCameraPosition
  (params (IndexCamera :type Integer))
  (bind _locationcamera (Variables|Default|GetLocationCamera))
  (bind _output_get (Variables|Default|SetIndexCamera (Math|Integer|Clamp(Integer) IndexCamera 0 (- (Utilities|Array|Length _locationcamera) 1))))
  (Transformation|SetActorTransform (Transformation|GetActorTransform (Utilities|Array|Get(acopy) _locationcamera _output_get)) true))

(event Custom|OnChangeTimeLine_Event)

(event Custom|CustomEvent
  (params (OldPawn :type Pawn%20Object%20Reference) (NewPawn :type Pawn%20Object%20Reference))
  (UserInterface|Viewport|AddtoViewport (Variables|/Game/ProtoMeca_2/Bureau_Enquête/Bureau/CharacterTest/BP_DeskTest_PC.BP_DeskTest_PC_C|GetCameraInterface (.AsBP%20Desk%20Test%20PC (Utilities|Casting|CastToBP_DeskTest_PC (Game|GetPlayerController 0)))) 0))

(event Input|EnhancedActionEvents|EnhancedInputActionIA_HintSelection
  (params (ActionValue :type Boolean) (ElapsedSeconds :type Float%20%28double-precision%29) (TriggeredSeconds :type Float%20%28double-precision%29) (InputAction :type Input%20Action%20Object%20Reference :default "/Game/ProtoMeca_2/CameraV2/Character/Input/Action/IA_HintSelection.IA_HintSelection"))
  (:Started
    (Utilities|FlowControl|Sequence
      (:then_0
        (bind _hitactor (CallFunction|MousePositiontoWorldLocation))
        (bind _asbp_hint_test (Utilities|Casting|CastToBP_HintTest _hitactor))
        (if (Variables|/Game/ProtoMeca_2/CameraV2/Hint/BP_HintTest.BP_HintTest_C|GetTypeHint _asbp_hint_test)
          (CallFunction|DisplayAnalyseOption "Visible")
          (else
            (CallFunction|DisplayAnalyseOption "Hidden")))))))

(event EventBeginPlay
  (Utilities|FlowControl|Sequence
    (:then_0
      (CallFunction|ChangeCameraPosition))
    (:then_1
      (Utilities|FlowControl|Delay 0.5)
      (bind _camerainterface (Utilities|GetCameraPlayerController))
      (EventDispatchers|BindEventtoOnChangeTimeLine _camerainterface (delegate Custom|OnChangeTimeLine_Event))
      (EventDispatchers|BindEventtoOnAudioFiltre _camerainterface (delegate Custom|AudioFiltre))
      (EventDispatchers|BindEventtoOnThermiqueFiltre _camerainterface (delegate Custom|ThermiqueFiltre))
      (EventDispatchers|BindEventtoOnUVFiltre _camerainterface (delegate Custom|UVFiltre))
      (EventDispatchers|BindEventtoNoFiltre _camerainterface (delegate Custom|NoFiltre)))
    (:then_2
      (Pawn|BindEventtoOnPossessedPawnChanged (Game|GetPlayerController 0) (delegate Custom|CustomEvent)))))

(fn ConstructionScript)

(fn DisplayAnalyseOption
  (params (InSetVisibility :type ESlateVisibility%20Enum :default "Visible"))
  (bind _camerainterface (Utilities|GetCameraPlayerController))
  (Widget|SetVisibility (Variables|/Game/ProtoMeca_2/CameraV2/Widget/WBP_CameraTest_Interface.WBP_CameraTest_Interface_C|GetAnalyseHint _camerainterface) InSetVisibility))

(fn MousePositiontoWorldLocation
  (bind _returnvalue (Game|GetPlayerController 0))
  (bind (_worldlocation _worlddirection) (Game|Player|ConvertMouseLocationToWorldSpace _returnvalue))
  (bind _outhit (Collision|LineTraceByChannel _worldlocation (+ _worldlocation (* _worlddirection 1e+03)) "TraceTypeQuery1" true 0 "ForDuration"))
  (return (.HitActor (Collision|BreakHitResult _outhit))))