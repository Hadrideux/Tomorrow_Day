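; BP_DataController is the search controller for the Dallas citizen database held in DT_CitoyenDallas.
; Recherche rebuilds CitoyensData by scanning every row, flattening administrative and personal fields into an array, and keeping citizens with any matching field.
; Matches are exact but case-insensitive, and empty searches match nothing.
; MAJDisplay separately forwards its input to the suspect data widget through the BP_CentreInformation_Test_PC player controller.
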(event Custom|Recherche
  (params (GetRecherche :type Text))
  (Utilities|Array|Clear (Variables|Default|GetCitoyensData))
  (bind _outrownames (CallFunction|GetDataRowName))
  (bind _array_element (Utilities|Array|ForEachLoopwithBreak _outrownames)
    (:LoopBody
      (bind (_array _returnvalue) (CallFunction|GetDataRow _array_element))
      (bind _array_element_2 (Utilities|Array|ForEachLoopwithBreak _array :!label _label)
        (:LoopBody
          (bind _searchcontains (CallFunction|SearchExistinData _array_element_2 GetRecherche))
          (if _searchcontains
            (Utilities|Array|Add (Variables|Default|GetCitoyensData) _returnvalue)
            (goto _label Break)))))))

(event Custom|MAJDisplay
  (params (GetSearch :type S%20Citoyens%20Data%20Structure))
  (bind _asbp_centre_information_test_pc (Utilities|Casting|CastToBP_CentreInformation_Test_PC (Game|GetPlayerController 0)))
  (Default|DisplaySearch (Variables|/Game/ProtoMeca_2/DataDallas/Widget/WBP_Recherche2.WBP_Recherche2_C|GetWBP_Suspect_Data (Variables|/Game/ProtoMeca_2/DataDallas/BP_CentreInformation_Test_PC.BP_CentreInformation_Test_PC_C|GetNewVar _asbp_centre_information_test_pc)) GetSearch))

(event EventBeginPlay)

(fn ConstructionScript)

(fn GetDataRow
  (params (RowName :type Name))
  (bind _returnvalue (Utilities|GetDataTableRow "/Game/ProtoMeca_2/DataDallas/DataBase/DT_CitoyenDallas.DT_CitoyenDallas" RowName)
    (:then
      (return (Utilities|Array|MakeArray (.NumérosIdentité (Utilities|Struct|BreakS_InformationAdministrativeData (.InformationAdministrative (Utilities|Struct|BreakS_CitoyensData _returnvalue)))) (.Nom (Utilities|Struct|BreakS_InformationAdministrativeData (.InformationAdministrative (Utilities|Struct|BreakS_CitoyensData _returnvalue)))) (.Prénom (Utilities|Struct|BreakS_InformationAdministrativeData (.InformationAdministrative (Utilities|Struct|BreakS_CitoyensData _returnvalue)))) (.LieuxNaissance (Utilities|Struct|BreakS_InformationAdministrativeData (.InformationAdministrative (Utilities|Struct|BreakS_CitoyensData _returnvalue)))) (.DateNaissance (Utilities|Struct|BreakS_InformationAdministrativeData (.InformationAdministrative (Utilities|Struct|BreakS_CitoyensData _returnvalue)))) (.Adresse (Utilities|Struct|BreakS_InformationAdministrativeData (.InformationAdministrative (Utilities|Struct|BreakS_CitoyensData _returnvalue)))) (.Sexe (Utilities|Struct|BreakS_InformationAdministrativeData (.InformationAdministrative (Utilities|Struct|BreakS_CitoyensData _returnvalue)))) (.Taille (Utilities|Struct|BreakS_InformationAdministrativeData (.InformationAdministrative (Utilities|Struct|BreakS_CitoyensData _returnvalue)))) (.DernierVote (Utilities|Struct|BreakS_InformationPersonnelData (.InformationPersonnel (Utilities|Struct|BreakS_CitoyensData _returnvalue)))) (.Travail (Utilities|Struct|BreakS_InformationPersonnelData (.InformationPersonnel (Utilities|Struct|BreakS_CitoyensData _returnvalue)))) (.Relation (Utilities|Struct|BreakS_InformationPersonnelData (.InformationPersonnel (Utilities|Struct|BreakS_CitoyensData _returnvalue)))) (.Affiliation (Utilities|Struct|BreakS_InformationPersonnelData (.InformationPersonnel (Utilities|Struct|BreakS_CitoyensData _returnvalue))))) _returnvalue))))

(fn GetDataRowName
  (bind _outrownames (DataTable|GetDataTableRowNames "/Game/ProtoMeca_2/DataDallas/DataBase/DT_CitoyenDallas.DT_CitoyenDallas"))
  (return _outrownames))

(fn SearchExistinData
  (params (RowData :type Text%20%28by%20ref%29) (Search :type Text%20%28by%20ref%29))
  (bind _returnvalue (Utilities|String|ToString(Text) Search))
  (bind _returnvalue_2 (Utilities|String|ToLower _returnvalue))
  (return (and (Utilities|Enum|Equal(Enum) (Utilities|String|ToLower (Utilities|String|ToString(Text) RowData)) _returnvalue_2) (not (Utilities|Array|IsEmpty _returnvalue_2)))))